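; BP_Source is an interactable inventory source actor whose mesh, name, type, value and description come from a data table row.
; The construction script applies that row, and BeginPlay copies name, type and value into its WB_Interaction widget.
; Interface events toggle custom-depth rendering on focus and route interaction to InteractOnServer, which flips InteractToggle.
; The OnRep for that toggle is still an empty stub.
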(event Custom|InteractOnServer
  (Variables|Default|SetInteractToggle (not (Variables|Default|GetInteractToggle))))

(event EventBeginPlay
  (bind _ref (CallFunction|GetInteractionWidgetRef))
  (bind _aswb_interaction (Utilities|Casting|CastToWB_Interaction (UserInterface|GetWidget _ref)))
  (bind _output_get (Variables|DONOTEDIT|SetWidgetRef _aswb_interaction))
  (Variables|/Game/StoryMap/UI/WB_Interaction.WB_Interaction_C|SetValueText _output_get (Variables|DONOTEDIT|GetValue))
  (Variables|/Game/StoryMap/UI/WB_Interaction.WB_Interaction_C|SetTypeText _output_get (Utilities|String|EnumtoString (Variables|DONOTEDIT|GetType)))
  (Variables|/Game/StoryMap/UI/WB_Interaction.WB_Interaction_C|SetNameText _output_get (Variables|DONOTEDIT|GetName)))

(event Collision|EventActorBeginOverlap
  (params (OtherActor :type Actor%20Object%20Reference)))

(event EventTick
  (params (DeltaSeconds :type Float%20%28single-precision%29)))

(event EventInterfaceToogleFocus
  (params (Focus :type Boolean))
  (Rendering|SetRenderCustomDepth (Variables|Default|GetStaticMesh) Focus))

(event EventInterfaceInteract
  (CallFunction|InteractonServer))

(fn ConstructionScript
  (bind _sourcedatatable (Variables|Edit|GetSourceDataTable))
  (bind _returnvalue (Utilities|GetDataTableRow (.datatable _sourcedatatable) (.rowname _sourcedatatable))
    (:then
      (bind _output_get (Variables|Edit|SetSource _returnvalue))
      (Variables|DONOTEDIT|SetMesh (.Mesh (Utilities|Struct|BreakF_SourceStruct _output_get)))
      (Variables|DONOTEDIT|SetName (.Name (Utilities|Struct|BreakF_SourceStruct _output_get)))
      (Variables|DONOTEDIT|SetType (.Type (Utilities|Struct|BreakF_SourceStruct _output_get)))
      (Variables|DONOTEDIT|SetValue (.Value (Utilities|Struct|BreakF_SourceStruct _output_get)))
      (Variables|DONOTEDIT|SetDescription (.Description (Utilities|Struct|BreakF_SourceStruct _output_get)))
      (Components|StaticMesh|SetStaticMesh (Variables|Default|GetStaticMesh) (Variables|DONOTEDIT|GetMesh)))))

(fn OnRepInteractToggle
  (if (Variables|Default|GetInteractToggle)
    _))

(fn GetInteractionWidgetRef
  (return (Variables|Default|GetWidget)))