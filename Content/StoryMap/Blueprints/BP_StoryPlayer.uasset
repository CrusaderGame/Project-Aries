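; BP_StoryPlayer is the story map's player pawn, moved by point-and-click.
; BeginPlay shows the mouse cursor on the first player controller.
; A left click runs a Visibility line trace from the deprojected cursor position and sends the pawn's controller to any hit with SimpleMoveToLocation.
; The trace end is built from the scaled cursor direction alone, without adding the start location.
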(event EventBeginPlay
  (Variables|/Script/Engine.PlayerController|SetbShowMouseCursor (Game|GetPlayerController 0) true))

(event Input|MouseEvents|LeftMouseButton
  (params (Key :type Key%20Structure :default "None"))
  (bind _returnvalue (Game|GetPlayerController 0))
  (bind (_worldlocation _worlddirection) (Game|Player|ConvertMouseLocationToWorldSpace _returnvalue))
  (:Pressed
    (bind (_outhit _returnvalue_2) (Collision|LineTraceByChannel _worldlocation (+ _worlddirection (* _worlddirection 1e+04)) "TraceTypeQuery1" false 0 "None"))
    (if _returnvalue_2
      (AI|Navigation|SimpleMovetoLocation (Pawn|GetController) (.Location (Collision|BreakHitResult _outhit))))))

(fn ConstructionScript)