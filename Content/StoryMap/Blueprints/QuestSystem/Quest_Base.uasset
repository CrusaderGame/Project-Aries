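; Base quest Blueprint that tracks objective progress for the current stage of a quest.
; On BeginPlay it loads its QuestID row from DT_Quest, zeroes a progress map keyed by the stage's objective IDs, and binds to the player controller's OnObjectiveIDCalled event.
; Each matching objective ID it hears raises that count by one, capped at the objective's required Quantity.
; Stage advancement and quest completion are not handled here.
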(event EventBeginPlay
  (CallFunction|GetQuestDetails)
  (EventDispatchers|BindEventtoOnObjectiveIDCalled (CallFunction|GetMyPlayerController) (EventDispatchers|CreateEvent :!event OnObjectiveIDHeard)))

(fn ConstructionScript)

(fn OnObjectiveIDHeard
  (params (ObjectiveID :type String))
  (bind _currentobcjectiveprogress (Variables|Default|GetCurrentObcjectiveProgress))
  (bind (_value _returnvalue) (Utilities|Map|Find _currentobcjectiveprogress ObjectiveID))
  (if _returnvalue
    (if (< _value (Utilities|Struct|BreakFObjectiveDetails (CallFunction|GetObjectiveDatabyID ObjectiveID)))
      (Utilities|Map|Add (Variables|Default|GetCurrentObcjectiveProgress) ObjectiveID (+ _value 1))
      (return))
    (else
      (return))))

(fn GetQuestDetails
  (bind _returnvalue (Utilities|GetDataTableRow "/Game/StoryMap/Blueprints/QuestSystem/Data/DT_Quest.DT_Quest" (Variables|Default|GetQuestID))
    (:then
      (bind _output_get (Variables|Default|SetQuestDetails _returnvalue))
      (bind _output_get_2 (Variables|Default|SetCurrentStageDetails (Utilities|Array|Get(acopy) (.Stages (Utilities|Struct|BreakFQuestDetails _output_get)) (Variables|Default|GetCurrentStage))))
      (Utilities|Map|Clear (Variables|Default|GetCurrentObcjectiveProgress))
      (for _array_element (Utilities|Struct|BreakFStageDetails _output_get_2)
        (Utilities|Map|Add (Variables|Default|GetCurrentObcjectiveProgress) (Utilities|Struct|BreakFObjectiveDetails _array_element) 0)))))

(fn GetObjectiveDatabyID
  (params (ObjectiveID :type String))
  (for _array_element (Utilities|Struct|BreakFStageDetails (Variables|Default|GetCurrentStageDetails))
    (if (Utilities|Enum|Equal(Enum) (Utilities|Struct|BreakFObjectiveDetails _array_element) ObjectiveID)
      (return _array_element))))