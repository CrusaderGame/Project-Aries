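; AC_QuestGiverComponent is an actor component that lets its owning actor act as a quest giver.
; InteractWith asks the player controller's quest log component whether the quest named by QuestData's row is active.
; If not, it calls DisplayQuest, which is still an empty stub; otherwise it prints an already-on-quest message.
; Both paths return the owner's display name, and the component does no work on BeginPlay or Tick.
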(event EventBeginPlay)

(event EventTick
  (params (DeltaSeconds :type Float%20%28single-precision%29)))

(fn DisplayQuest)

(fn Interactwith
  (bind _returnvalue (Components|GetOwner))
  (bind _returnvalue_2 (Utilities|GetDisplayName _returnvalue))
  (if (not (Default|QueryActiveQuest (Variables|/Game/StoryMap/Blueprints/Core/BP_StoryController.BP_StoryController_C|GetAC_QuestLogComponent (CallFunction|GetMyPlayerController)) (.rowname (Variables|Default|GetQuestData))))
    (CallFunction|DisplayQuest)
    (return _returnvalue_2)
    (else
      (Development|PrintString "Already on Quest")
      (return _returnvalue_2))))