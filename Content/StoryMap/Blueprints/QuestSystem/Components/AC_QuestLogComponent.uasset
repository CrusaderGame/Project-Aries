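; Actor component that serves as a quest log, tracking active quests.
; AddNewQuest records the quest ID uniquely, then spawns a Quest_Base actor with that ID, stores it in CurrentQuests and returns it.
; QueryActiveQuest checks whether an ID is in the active list.
; CompleteQuest and TrackQuest are empty stubs.
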(fn AddNewQuest
  (params (QuestID :type Name))
  (Utilities|Array|AddUnique (Variables|Default|GetCurrentActiveQuests) QuestID)
  (bind _returnvalue (Game|SpawnActorfromClass "/Game/StoryMap/Blueprints/QuestSystem/Quest_Base.Quest_Base_C" (Math|Transform|MakeTransform "0, 0, 0" "0, 0, 0" "1.000000,1.000000,1.000000") "Undefined" "MultiplyWithRoot" 0 QuestID 0))
  (Utilities|Array|Add (Variables|Default|GetCurrentQuests) _returnvalue)
  (return _returnvalue))

(fn CompleteQuest)

(fn QueryActiveQuest
  (params (QuestID :type Name))
  (return (Utilities|Array|ContainsItem (Variables|Default|GetCurrentActiveQuests) QuestID)))

(fn TrackQuest)