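; BL_CommonFunctionLibrary is a helper library for the StoryMap game that provides typed access to its core gameplay objects.
; Three getters fetch the player character and controller at index 0 and the current game mode.
; Each casts its result to BP_StoryPlayer, BP_StoryController or GM_StoryMap, with no handling for a failed cast.
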(fn GetMyPlayerCharacter
  (bind _asbp_story_player (Utilities|Casting|CastToBP_StoryPlayer (Game|GetPlayerCharacter 0)))
  (return _asbp_story_player))

(fn GetMyPlayerController
  (bind _asbp_story_controller (Utilities|Casting|CastToBP_StoryController (Game|GetPlayerController 0)))
  (return _asbp_story_controller))

(fn GetMyGameMode
  (bind _asgm_story_map (Utilities|Casting|CastToGM_StoryMap (Game|GetGameMode)))
  (return _asgm_story_map))