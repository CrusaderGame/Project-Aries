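; BP_StoryController is the player controller for story map mode, providing point-and-click movement, camera control and interaction.
; On BeginPlay it adds the Enhanced Input context, caches the BP_StoryPlayer pawn, creates the story UI, shows the cursor and enables interaction-trace ticking.
; Clicks trace under the cursor for SimpleMoveToLocation, while input drives clamped spring-arm zoom and yaw.
; Right mouse both gates rotation and toggles interaction; key 1 debug-prints Gold and Food.
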(event Input|EnhancedActionEvents|EnhancedInputActionIAStory_Zoom
  (params (ActionValue :type Float%20%28double-precision%29) (ElapsedSeconds :type Float%20%28double-precision%29) (TriggeredSeconds :type Float%20%28double-precision%29) (InputAction :type Input%20Action%20Object%20Reference :default "/Game/StoryMap/Blueprints/Core/Input/IAStory_Zoom.IAStory_Zoom"))
  (bind _camerazoomrange_min_max_ (Variables|CameraSettings|GetCameraZoomRange%28Min,Max%29))
  ;[0 0 0] CameraZoom
  (Variables|/Script/Engine.SpringArmComponent|SetTargetArmLength (Variables|/Game/StoryMap/Blueprints/Core/BP_StoryPlayer.BP_StoryPlayer_C|GetSpringArm (Variables|Default|GetCameraPawn)) (Math|Float|Clamp(Float) (+ (* (* ActionValue -1.0) (Variables|CameraSettings|GetCameraZoomSpeed)) (Variables|/Script/Engine.SpringArmComponent|GetTargetArmLength (Variables|/Game/StoryMap/Blueprints/Core/BP_StoryPlayer.BP_StoryPlayer_C|GetSpringArm (Variables|Default|GetCameraPawn)))) (.x _camerazoomrange_min_max_) (.y _camerazoomrange_min_max_))))

(event Input|EnhancedActionEvents|EnhancedInputActionIAStory_LookYaw
  (params (ActionValue :type Float%20%28double-precision%29) (ElapsedSeconds :type Float%20%28double-precision%29) (TriggeredSeconds :type Float%20%28double-precision%29) (InputAction :type Input%20Action%20Object%20Reference :default "/Game/StoryMap/Blueprints/Core/Input/IAStory_LookYaw.IAStory_LookYaw"))
  ;[0 0 0] CameraRotating
  (if (Game|Player|IsInputKeyDown "RightMouseButton")
    (Transformation|AddWorldRotation (Variables|/Game/StoryMap/Blueprints/Core/BP_StoryPlayer.BP_StoryPlayer_C|GetSpringArm (Variables|Default|GetCameraPawn)) (Math|Rotator|MakeRotator 0.0 0.0 (* ActionValue 3.0)) false false)))

(event Input|EnhancedActionEvents|EnhancedInputActionIAStory_Move
  (params (ActionValue :type Boolean) (ElapsedSeconds :type Float%20%28double-precision%29) (TriggeredSeconds :type Float%20%28double-precision%29) (InputAction :type Input%20Action%20Object%20Reference :default "/Game/StoryMap/Blueprints/Core/Input/IAStory_Move.IAStory_Move"))
  (bind _returnvalue (Game|GetPlayerController 0))
  (bind (_worldlocation _worlddirection) (Game|Player|ConvertMouseLocationToWorldSpace _returnvalue))
  ;[0 0 0] Point&Click
  (bind (_outhit _returnvalue_2) (Collision|LineTraceByChannel _worldlocation (+ _worlddirection (* _worlddirection 1e+05)) "TraceTypeQuery1" false 0 "None"))
  (if _returnvalue_2
    (AI|Navigation|SimpleMovetoLocation self (.Location (Collision|BreakHitResult _outhit)))))

(event EventBeginPlay
  (Utilities|Casting)
  (Transformation|SetWorldRotation (Variables|/Game/StoryMap/Blueprints/Core/BP_StoryPlayer.BP_StoryPlayer_C|GetSpringArm (Variables|Default|GetCameraPawn)) (Math|Rotator|MakeRotator 0.0 (* (Variables|CameraSettings|GetCameraPitch) -1.0) 0.0) false false)
  (Variables|/Script/Engine.PlayerController|SetbShowMouseCursor (Game|GetPlayerController 0) true)
  (CallFunction|SetupInteractionTrace))

(event Input|KeyboardEvents|1
  (params (Key :type Key%20Structure :default "None"))
  (:Pressed
    (Development|PrintString (Utilities|String|ToString(Integer) (Variables|Sources|GetGold)))
    (Development|PrintString (Utilities|String|ToString(Integer) (Variables|Sources|GetFood)) true true "(R=1.000000,G=0.000000,B=0.183826,A=1.000000)")))

(event Input|MouseEvents|RightMouseButton
  (params (Key :type Key%20Structure :default "None"))
  (bind _ac_interactiontrace (Variables|Default|GetAC_InteractionTrace))
  (:Pressed
    (Default|TrytoInteract _ac_interactiontrace true))
  (:Released
    (Default|TrytoInteract _ac_interactiontrace false)))

(fn ConstructionScript)

(fn SetArmLenght
  (Variables|/Script/Engine.SpringArmComponent|SetTargetArmLength (Variables|/Game/StoryMap/Blueprints/Core/BP_StoryPlayer.BP_StoryPlayer_C|GetSpringArm (Variables|Default|GetCameraPawn)) (Math|Float|Lerp 0.0 0.0 (Variables|CameraSettings|GetCameraZoomSpeed))))

(fn SetupInteractionTrace
  (Components|Tick|SetComponentTickEnabled (Variables|Default|GetAC_InteractionTrace) true))