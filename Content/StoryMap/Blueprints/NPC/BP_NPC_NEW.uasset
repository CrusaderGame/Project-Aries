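; Interactable NPC Blueprint that takes its type, name and skeletal mesh from a data table row in the construction script.
; At BeginPlay it fills the interaction widget with name and type, then hands its dialogue tree to its NPC_AI controller.
; Interface calls toggle custom depth on focus and route interaction through InteractOnServer, which flips InteractToogle and starts dialogue on the controller.
; The InteractToogle OnRep handler has no effect yet.
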(event Custom|InteractOnServer
  (Variables|Default|SetInteractToogle (not (Variables|Default|GetInteractToogle)))
  (bind _asnpc_ai (Utilities|Casting|CastToNPC_AI (AI|GetAIController self)))
  (Default|StartDialogue _asnpc_ai))

(event EventBeginPlay
  (bind _ref (CallFunction|GetInteractionWidgetRef))
  (bind _aswb_interaction_npc (Utilities|Casting|CastToWB_InteractionNPC (UserInterface|GetWidget _ref)))
  (bind _output_get (Variables|Default|SetWidgetRef _aswb_interaction_npc))
  (Variables|/Game/StoryMap/UI/WB_InteractionNPC.WB_InteractionNPC_C|SetNameText _output_get (Variables|Default|GetName))
  (Variables|/Game/StoryMap/UI/WB_InteractionNPC.WB_InteractionNPC_C|SetTypeText _output_get (Utilities|String|EnumtoString (Variables|Default|GetType)))
  (bind _asnpc_ai (Utilities|Casting|CastToNPC_AI (AI|GetAIController self)))
  (Variables|/Game/StoryMap/Blueprints/NPC/NPC_AI.NPC_AI_C|SetDialogueTree _asnpc_ai (Variables|Default|GetDialogueTree)))

(event EventInterfaceToogleFocus
  (params (Focus :type Boolean))
  (Rendering|SetRenderCustomDepth (Variables|Character|GetMesh) Focus))

(event EventInterfaceInteract
  (CallFunction|InteractonServer))

(fn ConstructionScript
  (bind _datatable (Variables|Default|GetDataTable))
  (bind _returnvalue (Utilities|GetDataTableRow (.datatable _datatable) (.rowname _datatable))
    (:then
      (bind _output_get (Variables|Default|SetNPC _returnvalue))
      (Variables|Default|SetType (.Type (Utilities|Struct|BreakF_NPCStruct _output_get)))
      (Variables|Default|SetName (.Name (Utilities|Struct|BreakF_NPCStruct _output_get)))
      (bind _output_get_2 (Variables|Default|SetCharacterMesh (.Mesh (Utilities|Struct|BreakF_NPCStruct _output_get))))
      (Components|SkeletalMesh|SetSkeletalMeshAsset (Variables|Character|GetMesh) _output_get_2))))

(fn OnRepInteractToogle
  (if (Variables|Default|GetInteractToogle)
    _))

(fn GetInteractionWidgetRef
  (return (Variables|Default|GetWidget)))