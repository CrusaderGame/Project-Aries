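; BP_SaveData stores and restores the player's quest state: active and completed quests plus per-quest progress.
; SaveQuestLog copies both quest lists from the quest log, while SaveQuestDetails records each quest's current stage and objective progress in a map keyed by quest ID.
; LoadQuests re-adds each active quest through the quest log component, restores its stage and progress from that map, then copies both lists back.
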(fn SaveQuestDetails
  (params (Quest :type Quest%20Base%20Object%20Reference))
  (Utilities|Map|Add (Variables|Default|GetQuestProgress) (Variables|/Game/StoryMap/Blueprints/QuestSystem/Quest_Base.Quest_Base_C|GetQuestID Quest) (Utilities|Struct|MakeFQuestSaveData (Variables|/Game/StoryMap/Blueprints/QuestSystem/Quest_Base.Quest_Base_C|GetCurrentObcjectiveProgress Quest) (Variables|/Game/StoryMap/Blueprints/QuestSystem/Quest_Base.Quest_Base_C|GetCurrentStage Quest))))

(fn LoadQuests
  (params (QuestLogComponent :type AC%20Quest%20Log%20Component%20Object%20Reference))
  (for _array_element (Variables|Default|GetCurrentActiveQuests)
    (bind _returnvalue (Default|AddNewQuest QuestLogComponent _array_element))
    (Variables|/Game/StoryMap/Blueprints/QuestSystem/Quest_Base.Quest_Base_C|SetCurrentStage _returnvalue (.CurrentStage (Utilities|Struct|BreakFQuestSaveData (.Value (Utilities|Map|Find (Variables|Default|GetQuestProgress) _array_element)))))
    (Variables|/Game/StoryMap/Blueprints/QuestSystem/Quest_Base.Quest_Base_C|SetCurrentObcjectiveProgress _returnvalue (.Progress (Utilities|Struct|BreakFQuestSaveData (.Value (Utilities|Map|Find (Variables|Default|GetQuestProgress) _array_element))))))
  (Variables|/Game/StoryMap/Blueprints/QuestSystem/Components/AC_QuestLogComponent.AC_QuestLogComponent_C|SetCurrentActiveQuests QuestLogComponent (Variables|Default|GetCurrentActiveQuests))
  (Variables|/Game/StoryMap/Blueprints/QuestSystem/Components/AC_QuestLogComponent.AC_QuestLogComponent_C|SetCompletedQuests QuestLogComponent (Variables|Default|GetCompletedQuests)))

(fn SaveQuestLog
  (params (QuestLog :type AC%20Quest%20Log%20Component%20Object%20Reference))
  (Variables|Default|SetCurrentActiveQuests (Variables|/Game/StoryMap/Blueprints/QuestSystem/Components/AC_QuestLogComponent.AC_QuestLogComponent_C|GetCurrentActiveQuests QuestLog))
  (Variables|Default|SetCompletedQuests (Variables|/Game/StoryMap/Blueprints/QuestSystem/Components/AC_QuestLogComponent.AC_QuestLogComponent_C|GetCompletedQuests QuestLog)))