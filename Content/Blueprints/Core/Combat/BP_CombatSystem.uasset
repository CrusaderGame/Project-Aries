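; Combat manager for a grid-based game that tracks units in combat, keeps tile occupancy in sync and casts spells.
; SetUnitIndexOnGrid updates both tiles and the unit's location as units are added, removed or reach new tiles.
; Grid generation and tile update events re-place units, destroying any on invalid tile types.
; CastSpell checks the target against the pattern-based range, then spawns the spell's animation actor with grid and target data.
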(event EventBeginPlay
  (EventDispatchers|BindEventtoOnGridGenerated (Variables|Default|GetGrid) (EventDispatchers|CreateEvent :!event OnGridGenerated))
  (EventDispatchers|BindEventtoOnTileDataUpdated (Variables|Default|GetGrid) (EventDispatchers|CreateEvent :!event OnTileDataUpdated)))

(event Collision|EventActorBeginOverlap
  (params (OtherActor :type Actor%20Object%20Reference)))

(event EventTick
  (params (DeltaSeconds :type Float%20%28single-precision%29)))

(fn ConstructionScript)

(fn AddUnitinCombat
  (params (Unit :type BP%20Unit%20Object%20Reference) (Index :type Int%20Point%20Structure))
  (Utilities|Array|Add (Variables|Default|GetUnitsInCombat) Unit)
  (CallFunction|SetUnitIndexonGrid Unit Index false)
  (Default|SetGrid Unit (Variables|Default|GetGrid))
  (EventDispatchers|BindEventtoOnUnitReachedNewTile Unit (EventDispatchers|CreateEvent :!event OnUnitReachedNewTile)))

(fn RemoveUnitfromCombat
  (params (Unit :type BP%20Unit%20Object%20Reference) (NewParam :type Boolean))
  (Utilities|Array|RemoveItem (Variables|Default|GetUnitsInCombat) Unit)
  (CallFunction|SetUnitIndexonGrid Unit (Utilities|Struct|MakeIntPoint -999 -999) false)
  (Actor|DestroyActor Unit))

(fn SetUnitIndexonGrid
  (params (Unit :type BP%20Unit%20Object%20Reference) (Index :type Int%20Point%20Structure) (Force :type Boolean))
  (Utilities|FlowControl|Sequence
    (:then_0
      (if (or (!= (Variables|/Game/Blueprints/Core/Units/BP_Unit.BP_Unit_C|GetIndex Unit) Index) Force)
        (Utilities|FlowControl|Sequence
          (:then_0
            (bind _output_get (LocalVariables|SetPreviousTile (.Value (Utilities|Map|Find (Variables|/Game/Blueprints/Core/Grid/BP_Grid.BP_Grid_C|GetGridTiles (Variables|Default|GetGrid)) (Variables|/Game/Blueprints/Core/Units/BP_Unit.BP_Unit_C|GetIndex Unit)))))
            (if (== (.UnitOnTile (Utilities|Struct|BreakS_TileData _output_get)) Unit)
              (bind _structout (Utilities|Struct|SetmembersinS_TileData (LocalVariables|GetPreviousTile) 0))
              (Utilities|Map|Add (Variables|/Game/Blueprints/Core/Grid/BP_Grid.BP_Grid_C|GetGridTiles (Variables|Default|GetGrid)) (.Index (Utilities|Struct|BreakS_TileData _structout)) _structout)))
          (:then_1
            (Variables|/Game/Blueprints/Core/Units/BP_Unit.BP_Unit_C|SetIndex Unit Index)
            (if (!= Index (Utilities|Struct|MakeIntPoint -999 -999))
              (bind _structout_2 (Utilities|Struct|SetmembersinS_TileData (.Value (Utilities|Map|Find (Variables|/Game/Blueprints/Core/Grid/BP_Grid.BP_Grid_C|GetGridTiles (Variables|Default|GetGrid)) Index)) Unit))
              (Utilities|Map|Add (Variables|/Game/Blueprints/Core/Grid/BP_Grid.BP_Grid_C|GetGridTiles (Variables|Default|GetGrid)) (.Index (Utilities|Struct|BreakS_TileData _structout_2)) _structout_2)))
          (:then_2
            (Default|CallOnUnitGridIndexChanged Unit)))))
    (:then_1
      (Transformation|SetActorLocation Unit (select (.ReturnValue (Utilities|Map|Find (Variables|/Game/Blueprints/Core/Grid/BP_Grid.BP_Grid_C|GetGridTiles (Variables|Default|GetGrid)) Index)) (.location (.Transform (Utilities|Struct|BreakS_TileData (.Value (Utilities|Map|Find (Variables|/Game/Blueprints/Core/Grid/BP_Grid.BP_Grid_C|GetGridTiles (Variables|Default|GetGrid)) Index))))) "-9999999.000000,-999999.000000,-999999.000000") false false))))

(fn OnGridGenerated
  (bind _output_get (LocalVariables|SetCopyOfUnitsInCombat (Variables|Default|GetUnitsInCombat)))
  (for _array_element _output_get
    (if (Utilities|Array|ContainsItem (.validtiletypes (.stats (Variables|/Game/Blueprints/Core/Units/BP_Unit.BP_Unit_C|GetUnitData _array_element))) (.type (.Value (Utilities|Map|Find (Variables|/Game/Blueprints/Core/Grid/BP_Grid.BP_Grid_C|GetGridTiles (Variables|Default|GetGrid)) (Variables|/Game/Blueprints/Core/Units/BP_Unit.BP_Unit_C|GetIndex _array_element)))))
      (CallFunction|SetUnitIndexonGrid _array_element (Variables|/Game/Blueprints/Core/Units/BP_Unit.BP_Unit_C|GetIndex _array_element) true)
      (else
        (CallFunction|RemoveUnitfromCombat _array_element false)))))

(fn OnTileDataUpdated
  (params (index :type Int%20Point%20Structure))
  (bind _output_get (LocalVariables|SetCopyOfUnitsInCombat (Variables|Default|GetUnitsInCombat)))
  (bind _array_element (Utilities|Array|ForEachLoopwithBreak _output_get :!label _label)
    (:LoopBody
      (if (Class|KismetMathLibrary|EqualIntPointIntPoint index (Variables|/Game/Blueprints/Core/Units/BP_Unit.BP_Unit_C|GetIndex _array_element))
        (if (Utilities|Array|ContainsItem (.validtiletypes (.stats (Variables|/Game/Blueprints/Core/Units/BP_Unit.BP_Unit_C|GetUnitData _array_element))) (.type (.Value (Utilities|Map|Find (Variables|/Game/Blueprints/Core/Grid/BP_Grid.BP_Grid_C|GetGridTiles (Variables|Default|GetGrid)) (Variables|/Game/Blueprints/Core/Units/BP_Unit.BP_Unit_C|GetIndex _array_element)))))
          (CallFunction|SetUnitIndexonGrid _array_element (Variables|/Game/Blueprints/Core/Units/BP_Unit.BP_Unit_C|GetIndex _array_element) false)
          (goto _label Break)
          (else
            (CallFunction|RemoveUnitfromCombat _array_element false)
            (goto _label Break)))))))

(fn OnUnitReachedNewTile
  (params (Unit :type BP%20Unit%20Object%20Reference) (Index :type Int%20Point%20Structure))
  (CallFunction|SetUnitIndexonGrid Unit Index false))

(fn CastSpell
  (params (Spell :type E_Spell%20Enum :default "NewEnumerator0") (OriginIndex :type Int%20Point%20Structure) (TargetIndex :type Int%20Point%20Structure))
  (bind _spelldata (CallFunction|GetSpellDatafromSpell Spell))
  (LocalVariables|SetData _spelldata)
  (bind _range_indexes (Spells|GetSpellRange OriginIndex (.Cast (Utilities|Struct|BreakS_SpellData (LocalVariables|GetData)))))
  (if (Utilities|Array|ContainsItem _range_indexes TargetIndex)
    (Game|SpawnActorfromClass (Utilities|Struct|BreakS_SpellData_Assets (.assets (LocalVariables|GetData))) (Math|Transform|MakeTransform "0.000000,0.000000,100.000000" "0, 0, 0" "1.000000,1.000000,1.000000") "AlwaysSpawn" "MultiplyWithRoot" 0 (Variables|Default|GetGrid) OriginIndex (Utilities|Array|MakeArray TargetIndex) 0)))

(fn GetSpellRange
  (params (Origin%20Index :type Int%20Point%20Structure) (Cast :type S%20Spell%20Data%20Cast%20Structure))
  (bind (_rangepattern _rangeminmax) (Utilities|Struct|BreakS_SpellData_Cast Cast))
  (bind _rangeindexes (CallFunction|GetIndexfromPatternandRange Origin%20Index (Variables|/Game/Blueprints/Core/Grid/BP_Grid.BP_Grid_C|GetGridShape (Variables|Default|GetGrid)) _rangepattern _rangeminmax))
  (return _rangeindexes))