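; Grid pathfinding Blueprint that runs an A*-style search between two tiles on square, hexagon or triangle grids, with optional diagonals.
; Neighbors are filtered by walkable type and height difference, then kept in a cost-sorted discovered list that favors non-diagonal steps on ties.
; Reaching the target rebuilds the path through previous-tile links.
; The search runs instantly or step by step through a delay gate, firing data-update, clear and completion callbacks.
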(event Custom|FindPathWithDelay
  (Utilities|FlowControl|Sequence
    (:then_0
      (goto _label_2 Open))
    (:then_1
      (if (> (Utilities|Array|Length (Variables|Default|GetDiscoveredTileIndexes)) 0) :!label _label
        (bind _foundtargettile (Pathfinding|AnalyseNextDiscoveredTile))
        (if _foundtargettile
          (bind _path (Pathfinding|GeneratePath))
          (Default|CallOnPathfindingCompleted _path)
          (else
            (Utilities|FlowControl|RetriggerableDelay (Variables|Default|GetDelayBetweenItterations))
            (Utilities|FlowControl|Gate true :!label _label_2
              (:Exit
                (goto _label)))))
        (else
          (Default|CallOnPathfindingCompleted (Utilities|Array|MakeArray)))))))

(event Custom|CloseDelayGate
  (Utilities|FlowControl|Gate true) ; enters at Close
)

(fn ConstructionScript)

(fn GetValidTileNeighbors
  (params (Index :type Int%20Point%20Structure) (IncludeDiagonals :type Boolean))
  (LocalVariables|SetInputData (.Value (Utilities|Map|Find (Variables|/Game/Blueprints/Core/Grid/BP_Grid.BP_Grid_C|GetGridTiles (Variables|Default|GetGrid)) Index)))
  (bind _neigbors (Neighbors|GetNeighborIndexes Index IncludeDiagonals))
  (for _array_element _neigbors
    (LocalVariables|SetData (.Value (Utilities|Map|Find (Variables|/Game/Blueprints/Core/Grid/BP_Grid.BP_Grid_C|GetGridTiles (Variables|Default|GetGrid)) _array_element)))
    (if (CallFunction|IsTileTypeWalkable (.type (LocalVariables|GetData)))
      (if (<= (Math|Float|Absolute(Float) (- (.z (.location (.transform (LocalVariables|GetData)))) (.z (.location (.transform (LocalVariables|GetInputData)))))) (.z (Variables|/Game/Blueprints/Core/Grid/BP_Grid.BP_Grid_C|GetGridTileSize (Variables|Default|GetGrid))))
        (Utilities|Array|Add (LocalVariables|GetRet) (Utilities|Struct|MakeS_PathfindingData (.index (LocalVariables|GetData)) 1 99999999 99999999 Index)))))
  (return (LocalVariables|GetRet)))

(fn GetNeighborsIndexesforSquare
  (params (Index :type Int%20Point%20Structure) (IncludeDiagonals :type Boolean))
  (bind _intpoint (Utilities|Struct|MakeIntPoint 1 0))
  (bind _intpoint_2 (Utilities|Struct|MakeIntPoint 0 1))
  (bind _intpoint_3 (Utilities|Struct|MakeIntPoint -1 0))
  (bind _intpoint_4 (Utilities|Struct|MakeIntPoint 0 -1))
  (bind _returnvalue (+ Index _intpoint))
  (bind _returnvalue_2 (+ Index _intpoint_2))
  (bind _returnvalue_3 (+ Index _intpoint_3))
  (bind _returnvalue_4 (+ Index _intpoint_4))
  (bind _array (Utilities|Array|MakeArray _returnvalue _returnvalue_2 _returnvalue_3 _returnvalue_4))
  (if IncludeDiagonals
    (LocalVariables|SetRet _array)
    (Utilities|Array|AppendArray (LocalVariables|GetRet) (Utilities|Array|MakeArray (+ Index (Utilities|Struct|MakeIntPoint 1 1)) (+ Index (Utilities|Struct|MakeIntPoint -1 1)) (+ Index (Utilities|Struct|MakeIntPoint -1 -1)) (+ Index (Utilities|Struct|MakeIntPoint 1 -1))))
    (return (LocalVariables|GetRet))
    (else
      (return _array))))

(fn GetNeighborsIndexesforHexagone
  (params (Index :type Int%20Point%20Structure))
  (return (Utilities|Array|MakeArray (+ Index (Utilities|Struct|MakeIntPoint 1 1)) (+ Index (Utilities|Struct|MakeIntPoint 0 2)) (+ Index (Utilities|Struct|MakeIntPoint -1 1)) (+ Index (Utilities|Struct|MakeIntPoint -1 -1)) (+ Index (Utilities|Struct|MakeIntPoint 0 -2)) (+ Index (Utilities|Struct|MakeIntPoint 1 -1)))))

(fn GetNeighborsIndexesforTriangle
  (params (Index :type Int%20Point%20Structure) (IncludeDiagonals :type Boolean))
  (LocalVariables|SetRet (Utilities|Array|MakeArray (+ Index (Utilities|Struct|MakeIntPoint 0 -1)) (+ Index (Utilities|Struct|MakeIntPoint 0 1))))
  (if (== (CallFunction|IsIntEven (.x Index)) (CallFunction|IsIntEven (.y Index)))
    (Utilities|Array|Add (LocalVariables|GetRet) (+ Index (Utilities|Struct|MakeIntPoint -1 0)))
    (else
      (Utilities|Array|Add (LocalVariables|GetRet) (+ Index (Utilities|Struct|MakeIntPoint 1 0)))))
  (if IncludeDiagonals
    (if (== (CallFunction|IsIntEven (.x Index)) (CallFunction|IsIntEven (.y Index)))
      (Utilities|Array|AppendArray (LocalVariables|GetRet) (Utilities|Array|MakeArray (+ Index (Utilities|Struct|MakeIntPoint 1 0)) (+ Index (Utilities|Struct|MakeIntPoint -1 2)) (+ Index (Utilities|Struct|MakeIntPoint -1 -2))))
      (else
        (Utilities|Array|AppendArray (LocalVariables|GetRet) (Utilities|Array|MakeArray (+ Index (Utilities|Struct|MakeIntPoint -1 0)) (+ Index (Utilities|Struct|MakeIntPoint 1 2)) (+ Index (Utilities|Struct|MakeIntPoint 1 -2))))))
    (return (LocalVariables|GetRet))
    (else
      (return (LocalVariables|GetRet)))))

(fn GetNeighborIndexes
  (params (Index :type Int%20Point%20Structure) (IncludeDiagonals :type Boolean))
  (switch Utilities|FlowControl|Switch|SwitchonE_GridShapes (Variables|/Game/Blueprints/Core/Grid/BP_Grid.BP_Grid_C|GetGridShape (Variables|Default|GetGrid))
    (:NewEnumerator0
      (return (Neighbors|GetNeighborsIndexesforSquare Index IncludeDiagonals)))
    (:NewEnumerator1
      (return (Neighbors|GetNeighborsIndexesforHexagone Index)))
    (:NewEnumerator2
      (return (Neighbors|GetNeighborsIndexesforTriangle Index IncludeDiagonals)))))

(fn FindPath
  (params (Start :type Int%20Point%20Structure) (Target :type Int%20Point%20Structure) (Diagonals :type Boolean) (Delay :type Float%20%28double-precision%29))
  (bind _array (Utilities|Array|MakeArray ""))
  (bind _array_2 (Utilities|Array|MakeArray ""))
  (Variables|Default|SetStartIndex Start)
  (Variables|Default|SetTargetIndex Target)
  (Variables|Default|SetInclude%20Diagonals Diagonals)
  (Variables|Default|SetDelayBetweenItterations Delay)
  (CallFunction|CloseDelayGate)
  (CallFunction|ClearGeneratedData)
  (bind _isvalid (Pathfinding|IsInputDataValid))
  (if _isvalid
    (Pathfinding|DiscoverTile (Utilities|Struct|MakeS_PathfindingData (Variables|Default|GetStartIndex) 1 0 (Pathfinding|GetMinimumCostBetweenTwoTiles (Variables|Default|GetStartIndex) (Variables|Default|GetTargetIndex) (Variables|Default|GetInclude%20Diagonals)) "(X=-999,Y=-999)"))
    (if (<= (Variables|Default|GetDelayBetweenItterations) 0.0)
      (while (> (Utilities|Array|Length (Variables|Default|GetDiscoveredTileIndexes)) 0)
        (bind _foundtargettile (Pathfinding|AnalyseNextDiscoveredTile))
        (if _foundtargettile
          (bind _path (Pathfinding|GeneratePath))
          (Default|CallOnPathfindingCompleted _path)
          (return _path)))
      (Default|CallOnPathfindingCompleted _array_2)
      (return _array_2)
      (else
        (CallFunction|FindPathwithDelay)
        (return (Utilities|Array|MakeArray ""))))
    (else
      (Default|CallOnPathfindingCompleted _array)
      (return _array))))

(fn IsInputDataValid
  (if (!= (Variables|Default|GetStartIndex) (Variables|Default|GetTargetIndex))
    (if (Default|IsTileWalkable (Variables|Default|GetGrid) (Variables|Default|GetStartIndex))
      (if (Default|IsTileWalkable (Variables|Default|GetGrid) (Variables|Default|GetTargetIndex))
        (return true)
        (else
          (return false)))
      (else
        (return false)))
    (else
      (return false))))

(fn DiscoverTile
  (params (TilePathData :type S%20Pathfinding%20Data%20Structure))
  (bind _index (Utilities|Struct|BreakS_PathfindingData TilePathData))
  ;[0 0 0] Add tile into data and inside the Discovered lists
  (Utilities|Map|Add (Variables|Default|GetPathfindingData) _index TilePathData)
  (Pathfinding|InsertTileinDiscoveredArray TilePathData)
  (Default|CallOnPathfindingDataUpdated _index))

(fn GetMinimumCostBetweenTwoTiles
  (params (Index1 :type Int%20Point%20Structure) (Index2 :type Int%20Point%20Structure) (Diagonals :type Boolean))
  (bind _returnvalue (- Index1 Index2))
  (bind _returnvalue_2 (- Index1 Index2))
  (bind _returnvalue_3 (< (.x Index2) (.x Index1)))
  (bind _returnvalue_4 (< (.x Index2) (.x Index1)))
  (bind _returnvalue_5 (- Index1 Index2))
  (bind _returnvalue_6 (- Index1 Index2))
  (bind _returnvalue_7 (- Index1 Index2))
  (bind _returnvalue_8 (Math|Integer|Absolute(Integer) (.x _returnvalue_6)))
  (bind _returnvalue_9 (select _returnvalue_4 -1 1))
  (switch Utilities|FlowControl|Switch|SwitchonE_GridShapes (Variables|/Game/Blueprints/Core/Grid/BP_Grid.BP_Grid_C|GetGridShape (Variables|Default|GetGrid))
    (:NewEnumerator0
      (if Diagonals
        (return (Math|Integer|Max(Integer) (Math|Integer|Absolute(Integer) (.x _returnvalue_2)) (Math|Integer|Absolute(Integer) (.y _returnvalue_2))))
        (else
          (return (+ (Math|Integer|Absolute(Integer) (.x _returnvalue_5)) (Math|Integer|Absolute(Integer) (.y _returnvalue_5)))))))
    (:NewEnumerator1
      (return (+ _returnvalue_8 (Math|Integer|Max(Integer) (/ (- (Math|Integer|Absolute(Integer) (.y _returnvalue_6)) _returnvalue_8) 2)))))
    (:NewEnumerator2
      (if Diagonals
        (return (+ (Math|Integer|Absolute(Integer) (.x _returnvalue)) (Math|Integer|Absolute(Integer) (.y _returnvalue))))
        (else
          (LocalVariables|SetX (Math|Integer|Absolute(Integer) (.x _returnvalue_7)))
          (LocalVariables|SetY (Math|Integer|Absolute(Integer) (.y _returnvalue_7)))
          (if (select (== (CallFunction|IsIntEven (.x Index1)) (CallFunction|IsIntEven (.y Index1))) (select _returnvalue_3 (<= (- (LocalVariables|GetX) 1) (LocalVariables|GetY)) (<= (LocalVariables|GetX) (LocalVariables|GetY))) (select _returnvalue_3 (<= (LocalVariables|GetX) (LocalVariables|GetY)) (<= (- (LocalVariables|GetX) 1) (LocalVariables|GetY))))
            (return (+ (LocalVariables|GetX) (LocalVariables|GetY)))
            (elif (== (CallFunction|IsIntEven (LocalVariables|GetX)) (CallFunction|IsIntEven (LocalVariables|GetY)))
              (return (* (LocalVariables|GetX) 2))
              (else
                (return (+ (* (LocalVariables|GetX) 2) (select (== (CallFunction|IsIntEven (.x Index1)) (CallFunction|IsIntEven (.y Index1))) _returnvalue_9 (* _returnvalue_9 -1))))))))))))

(fn AnalyseNextDiscoveredTile
  (bind _tilepathdata (Pathfinding|PullCheapestTileOutOfDiscoeredList))
  (Variables|Default|SetCurrentDiscoveredTile _tilepathdata)
  (bind _neigbors (Neighbors|GetValidTileNeighbors (.Index (Utilities|Struct|BreakS_PathfindingData (Variables|Default|GetCurrentDiscoveredTile))) (Variables|Default|GetInclude%20Diagonals)))
  (Variables|Default|SetCurrentNeigbors _neigbors)
  (while (> (Utilities|Array|Length (Variables|Default|GetCurrentNeigbors)) 0)
    (bind _istargettile (Pathfinding|DiscoverNextNeighbor))
    (if _istargettile
      (return true)))
  (return false))

(fn GeneratePath
  ;[0 0 0] Retrieve the path from the TargetIndex back to StartIndex. Then reverse it so it's in the right way
  (LocalVariables|SetCurrent (Variables|Default|GetTargetIndex))
  (while (!= (LocalVariables|GetCurrent) (Variables|Default|GetStartIndex))
    (Utilities|Array|Add (LocalVariables|GetInvertedPath) (LocalVariables|GetCurrent))
    (LocalVariables|SetCurrent (.PreviousIndex (Utilities|Struct|BreakS_PathfindingData (.Value (Utilities|Map|Find (Variables|Default|GetPathfindingData) (LocalVariables|GetCurrent)))))))
  (bind _arrayelement (Utilities|Array|ReverseforEachLoop (LocalVariables|GetInvertedPath))
    (:LoopBody
      (Utilities|Array|Add (LocalVariables|GetRet) _arrayelement))
    (:Completed
      (return (LocalVariables|GetRet)))))

(fn PullCheapestTileOutOfDiscoeredList
  (LocalVariables|SetTileIndex (Utilities|Array|Get(acopy) (Variables|Default|GetDiscoveredTileIndexes)))
  (Utilities|Array|RemoveIndex (Variables|Default|GetDiscoveredTileSortingCost))
  (Utilities|Array|RemoveIndex (Variables|Default|GetDiscoveredTileIndexes))
  (Utilities|Array|Add (Variables|Default|GetAnalysedTileIndex) (LocalVariables|GetTileIndex))
  (return (.Value (Utilities|Map|Find (Variables|Default|GetPathfindingData) (LocalVariables|GetTileIndex)))))

(fn DiscoverNextNeighbor
  (Variables|Default|SetCurrentNeighbor (Utilities|Array|Get(acopy) (Variables|Default|GetCurrentNeigbors)))
  (Utilities|Array|RemoveIndex (Variables|Default|GetCurrentNeigbors))
  (if (not (Utilities|Array|ContainsItem (Variables|Default|GetAnalysedTileIndex) (.Index (Utilities|Struct|BreakS_PathfindingData (Variables|Default|GetCurrentNeighbor)))))
    (LocalVariables|SetCostFromStart (+ (.CostToEnterTile (Utilities|Struct|BreakS_PathfindingData (Variables|Default|GetCurrentDiscoveredTile))) (.CostToEnterTile (Utilities|Struct|BreakS_PathfindingData (Variables|Default|GetCurrentNeighbor)))))
    (bind _output_get (LocalVariables|SetIndexInDiscovered (Utilities|Array|FindItem (Variables|Default|GetDiscoveredTileIndexes) (.Index (Utilities|Struct|BreakS_PathfindingData (Variables|Default|GetCurrentNeighbor))))))
    (if (== _output_get -1)
      _
      (else
        (bind _output_get_2 (Variables|Default|SetCurrentNeighbor (.Value (Utilities|Map|Find (Variables|Default|GetPathfindingData) (.Index (Utilities|Struct|BreakS_PathfindingData (Variables|Default|GetCurrentNeighbor)))))))
        (if (< (LocalVariables|GetCostFromStart) (.CostToEnterTile (Utilities|Struct|BreakS_PathfindingData _output_get_2)))
          (Utilities|Array|RemoveIndex (Variables|Default|GetDiscoveredTileIndexes) (LocalVariables|GetIndexInDiscovered))
          (Utilities|Array|RemoveIndex (Variables|Default|GetDiscoveredTileSortingCost) (LocalVariables|GetIndexInDiscovered))
          (else
            (return false)))))
    (Pathfinding|DiscoverTile (Utilities|Struct|MakeS_PathfindingData (.Index (Utilities|Struct|BreakS_PathfindingData (Variables|Default|GetCurrentNeighbor))) (.CostToEnterTile (Utilities|Struct|BreakS_PathfindingData (Variables|Default|GetCurrentNeighbor))) (LocalVariables|GetCostFromStart) (Pathfinding|GetMinimumCostBetweenTwoTiles (.Index (Utilities|Struct|BreakS_PathfindingData (Variables|Default|GetCurrentNeighbor))) (Variables|Default|GetTargetIndex) (Variables|Default|GetInclude%20Diagonals)) (.Index (Utilities|Struct|BreakS_PathfindingData (Variables|Default|GetCurrentDiscoveredTile)))))
    (if (Class|KismetMathLibrary|EqualIntPointIntPoint (.Index (Utilities|Struct|BreakS_PathfindingData (Variables|Default|GetCurrentNeighbor))) (Variables|Default|GetTargetIndex))
      (return true)
      (else
        (return false)))
    (else
      (return false))))

(fn InsertTileinDiscoveredArray
  (params (TileData :type S%20Pathfinding%20Data%20Structure))
  (bind _discoveredtilesortingcost (Variables|Default|GetDiscoveredTileSortingCost))
  ;[0 0 0] Insert the tile in the right position in the array. Sorting it from Cheapest to MostExpensive. That way, next time we try to find the cheapest tile, we can simply take the index 0.
  (LocalVariables|SetSourtingCost (CallFunction|GetTileSortingCost TileData))
  (if (== (Utilities|Array|Length (Variables|Default|GetDiscoveredTileSortingCost)) 0)
    (Utilities|Array|Add (Variables|Default|GetDiscoveredTileSortingCost) (LocalVariables|GetSourtingCost) :!label _label)
    (Utilities|Array|Add (Variables|Default|GetDiscoveredTileIndexes) (.Index (Utilities|Struct|BreakS_PathfindingData TileData)))
    (elif (>= (LocalVariables|GetSourtingCost) (Utilities|Array|Get(acopy) _discoveredtilesortingcost (Utilities|Array|LastIndex _discoveredtilesortingcost)))
      (goto _label)
      (else
        (bind (_array_element _array_index) (Utilities|Array|ForEachLoopwithBreak (Variables|Default|GetDiscoveredTileSortingCost) :!label _label_2)
          (:LoopBody
            (if (>= _array_element (LocalVariables|GetSourtingCost))
              (Utilities|Array|Insert (Variables|Default|GetDiscoveredTileSortingCost) (LocalVariables|GetSourtingCost) _array_index)
              (Utilities|Array|Insert (Variables|Default|GetDiscoveredTileIndexes) (.Index (Utilities|Struct|BreakS_PathfindingData TileData)) _array_index)
              (goto _label_2 Break))))))))

(fn ClearGeneratedData
  ;[0 0 0] Just clear everything so we start every pathfinding clean
  (Utilities|Map|Clear (Variables|Default|GetPathfindingData))
  (Utilities|Array|Clear (Variables|Default|GetDiscoveredTileSortingCost))
  (Utilities|Array|Clear (Variables|Default|GetDiscoveredTileIndexes))
  (Utilities|Array|Clear (Variables|Default|GetAnalysedTileIndex))
  (Default|CallOnPathfindingDataCleared))

(fn IsDiagonal
  (params (Index1 :type Int%20Point%20Structure) (Index2 :type Int%20Point%20Structure))
  (bind _neigbors (Neighbors|GetNeighborIndexes Index1 false))
  (return (not (Utilities|Array|ContainsItem _neigbors Index2))))

(fn GetTileSortingCost
  (params (S_PathfindingData :type S%20Pathfinding%20Data%20Structure%20%28by%20ref%29))
  (bind (_index _costtoentertile _costfromstart _minimumcosttotarget) (Utilities|Struct|BreakS_PathfindingData S_PathfindingData))
  (bind (_index_2 _costtoentertile_2 _costfromstart_2 _minimumcosttotarget_2 _previousindex) (Utilities|Struct|BreakS_PathfindingData S_PathfindingData))
  (return (+ (* (+ _costfromstart _minimumcosttotarget) 2) (CallFunction|IsDiagonal _index_2 _previousindex))))