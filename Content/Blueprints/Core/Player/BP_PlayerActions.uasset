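; Player input actor for the tile grid that tracks the hovered and selected tile and unit and runs swappable left and right click actions.
; Tick traces for a unit, falling back to the grid tile, and updates hover states.
; Spawned action actors execute on press and on each newly hovered tile while the button is held.
; Grid and combat system events keep the selection in sync.
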(event Custom|OnHoveredTileChanged
  (bind _selectedaction_rightcilck (Variables|Default|GetSelectedAction_RightCilck))
  (bind _selectedaction_leftcilck (Variables|Default|GetSelectedAction_LeftCilck))
  ;[0 0 0] If the player Left Clicks, we execute the LeftClickAction and same thing for the Right Click. If the player Right Clicks, we execute the RightClickAction
  ; And we also execute the action if the player keep the mouse button down and move his mouse hover different tiles.
  (Utilities|FlowControl|Sequence
    (:then_0
      (Utilities|IsValid _selectedaction_leftcilck
        (:Is%20Valid
          (Default|ExecuteHoveredAction _selectedaction_leftcilck (Variables|Default|GetHoveredTile))
          (if (Variables|Default|GetIsLeftClickDown)
            (Default|ExecuteAction (Variables|Default|GetSelectedAction_LeftCilck) (Variables|Default|GetHoveredTile))))))
    (:then_1
      (Utilities|IsValid _selectedaction_rightcilck
        (:Is%20Valid
          (Default|ExecuteHoveredAction _selectedaction_rightcilck (Variables|Default|GetHoveredTile))
          (if (Variables|Default|GetIsRightClickDown)
            (Default|ExecuteAction (Variables|Default|GetSelectedAction_RightCilck) (Variables|Default|GetHoveredTile))))))))

(event EventBeginPlay
  (bind _returnvalue (Actor|GetActorOfClass "/Game/Blueprints/Core/Grid/BP_Grid.BP_Grid_C"))
  (Variables|References|SetGrid _returnvalue)
  (EventDispatchers|BindEventtoOnGridGenerated (Variables|References|GetGrid) (EventDispatchers|CreateEvent :!event OnGridGenerated))
  (EventDispatchers|BindEventtoOnTileDataUpdated (Variables|References|GetGrid) (EventDispatchers|CreateEvent :!event OnTileDataUpdated))
  (bind _returnvalue_2 (Actor|GetActorOfClass "/Game/Blueprints/Core/Combat/BP_CombatSystem.BP_CombatSystem_C"))
  (bind _output_get (Variables|Default|SetCombatSystem _returnvalue_2))
  (EventDispatchers|BindEventtoOnUnitGridIndexChanged _output_get (EventDispatchers|CreateEvent :!event OnUnitGridIndexChanged))
  (Input|EnableInput (Game|GetPlayerController 0))
  (CallFunction|SetSelectedActions "/Game/Blueprints/Core/Player/Actions/Grid/Action_SelectTileAndUnit.Action_SelectTileAndUnit_C" "/Game/Blueprints/Core/Player/Actions/Grid/Action_SelectTileAndUnit.Action_SelectTileAndUnit_C"))

(event EventTick
  (params (DeltaSeconds :type Float%20%28single-precision%29))
  (CallFunction|UpdateHoveredTileandUnit))

(event Input|MouseEvents|LeftMouseButton
  (params (Key :type Key%20Structure :default "None"))
  ;[0 0 0] If the player Left Clicks, we execute the LeftClickAction and same thing for the Right Click. If the player Right Clicks, we execute the RightClickAction
  ; And we also execute the action if the player keep the mouse button down and move his mouse hover different tiles.
  (:Pressed
    (CallFunction|UpdateHoveredTileandUnit)
    (Variables|Default|SetIsLeftClickDown true)
    (Utilities|IsValid (Variables|Default|GetSelectedAction_LeftCilck)
      (:Is%20Valid
        (Default|ExecuteAction (Variables|Default|GetSelectedAction_LeftCilck) (Variables|Default|GetHoveredTile)))))
  (:Released
    (Variables|Default|SetIsLeftClickDown false)))

(event Input|MouseEvents|RightMouseButton
  (params (Key :type Key%20Structure :default "None"))
  ;[0 0 0] If the player Left Clicks, we execute the LeftClickAction and same thing for the Right Click. If the player Right Clicks, we execute the RightClickAction
  ; And we also execute the action if the player keep the mouse button down and move his mouse hover different tiles.
  (:Pressed
    (CallFunction|UpdateHoveredTileandUnit)
    (Variables|Default|SetIsRightClickDown true)
    (Utilities|IsValid (Variables|Default|GetSelectedAction_RightCilck)
      (:Is%20Valid
        (Default|ExecuteAction (Variables|Default|GetSelectedAction_RightCilck) (Variables|Default|GetHoveredTile)))))
  (:Released
    (Variables|Default|SetIsRightClickDown false)))

(fn ConstructionScript)

(fn UpdateHoveredTileandUnit
  (Utilities|FlowControl|Sequence
    (:then_0
      (bind _unit (CallFunction|GetUnitUnderCursor))
      (if (!= _unit (Variables|Default|GetHoveredUnit))
        (Utilities|FlowControl|Sequence
          (:then_0
            (Utilities|IsValid (Variables|Default|GetHoveredUnit)
              (:Is%20Valid
                (Default|SetIsHovered (Variables|Default|GetHoveredUnit) false))))
          (:then_1
            (bind _output_get (Variables|Default|SetHoveredUnit _unit))
            (Utilities|IsValid _output_get
              (:Is%20Valid
                (Default|SetIsHovered _output_get true)))))))
    (:then_1
      (Utilities|IsValid (Variables|Default|GetHoveredUnit)
        (:Is%20Valid
          (LocalVariables|SetNewIndex (Variables|/Game/Blueprints/Core/Units/BP_Unit.BP_Unit_C|GetIndex (Variables|Default|GetHoveredUnit))))
        (:Is%20Not%20Valid
          (bind _index (Default|GetTileIndexUnderCursor (Variables|References|GetGrid)))
          (LocalVariables|SetNewIndex _index)))
      (if (!= (LocalVariables|GetNewIndex) (Variables|Default|GetHoveredTile))
        (Default|RemoveStatefromTile (Variables|References|GetGrid) (Variables|Default|GetHoveredTile) "NewEnumerator1")
        (Variables|Default|SetHoveredTile (LocalVariables|GetNewIndex))
        (Default|AddStatetoTile (Variables|References|GetGrid) (Variables|Default|GetHoveredTile) "NewEnumerator1")
        (CallFunction|OnHoveredTileChanged)))))

(fn SetSelectedActions
  (params (LeftAction :type BP%20Action%20Class%20Reference) (RightAction :type BP%20Action%20Class%20Reference))
  (Utilities|FlowControl|Sequence
    (:then_0
      (Utilities|IsValid (Variables|Default|GetSelectedAction_LeftCilck)
        (:Is%20Valid
          (Actor|DestroyActor (Variables|Default|GetSelectedAction_LeftCilck))
          (Variables|Default|SetSelectedAction_LeftCilck 0))
        (:Is%20Not%20Valid
          _))
      (if (Utilities|IsValidClass LeftAction)
        (bind _returnvalue (Game|SpawnActorfromClass LeftAction (Math|Transform|MakeTransform "0, 0, 0" "0, 0, 0" "1.000000,1.000000,1.000000") "AlwaysSpawn" "MultiplyWithRoot" 0 self 0))
        (Variables|Default|SetSelectedAction_LeftCilck _returnvalue)))
    (:then_1
      (Utilities|IsValid (Variables|Default|GetSelectedAction_RightCilck)
        (:Is%20Valid
          (Actor|DestroyActor (Variables|Default|GetSelectedAction_RightCilck))
          (Variables|Default|SetSelectedAction_RightCilck 0))
        (:Is%20Not%20Valid
          _))
      (if (Utilities|IsValidClass RightAction)
        (bind _returnvalue_2 (Game|SpawnActorfromClass RightAction (Math|Transform|MakeTransform "0, 0, 0" "0, 0, 0" "1.000000,1.000000,1.000000") "AlwaysSpawn" "MultiplyWithRoot" 0 self 0))
        (Variables|Default|SetSelectedAction_RightCilck _returnvalue_2)))
    (:then_2
      (Default|CallOnSelectedActionsChanged (Variables|Default|GetSelectedAction_LeftCilck) (Variables|Default|GetSelectedAction_RightCilck)))))

(fn GetUnitUnderCursor
  (params (PlayerIndex :type Integer))
  (bind _returnvalue (Game|GetPlayerController PlayerIndex))
  (bind (_hitresult _returnvalue_2) (Game|Player|GetHitResultUnderCursorbyChannel _returnvalue "TraceTypeQuery5" false))
  (if _returnvalue_2
    (return (.AsBP%20Unit (Utilities|Casting|CastToBP_Unit (.HitActor (Collision|BreakHitResult _hitresult)))))
    (else
      (bind _index (Default|GetTileIndexUnderCursor (Variables|References|GetGrid) PlayerIndex))
      (return (.UnitOnTile (Utilities|Struct|BreakS_TileData (.Value (Utilities|Map|Find (Variables|/Game/Blueprints/Core/Grid/BP_Grid.BP_Grid_C|GetGridTiles (Variables|References|GetGrid)) _index))))))))

(fn SetSelectedTileandUnit
  (params (Index :type Int%20Point%20Structure) (Force :type Boolean))
  (Utilities|FlowControl|Sequence
    (:then_0
      (if (or (!= (Variables|Default|GetSelectedTile) Index) Force)
        (Default|RemoveStatefromTile (Variables|References|GetGrid) (Variables|Default|GetSelectedTile) "NewEnumerator2")
        (Variables|Default|SetSelectedTile Index)
        (Default|AddStatetoTile (Variables|References|GetGrid) (Variables|Default|GetSelectedTile) "NewEnumerator2")
        (else
          (Default|RemoveStatefromTile (Variables|References|GetGrid) (Variables|Default|GetSelectedTile) "NewEnumerator2")
          (Variables|Default|SetSelectedTile (Utilities|Struct|MakeIntPoint -999 -999))))
      (Default|CallOnSelectedTileChanged Index))
    (:then_1
      (LocalVariables|SetNewUnit (.UnitOnTile (Utilities|Struct|BreakS_TileData (.Value (Utilities|Map|Find (Variables|/Game/Blueprints/Core/Grid/BP_Grid.BP_Grid_C|GetGridTiles (Variables|References|GetGrid)) (Variables|Default|GetSelectedTile))))))
      (if (or (!= (Variables|Default|GetSelectedUnit) (LocalVariables|GetNewUnit)) Force)
        (Utilities|FlowControl|Sequence
          (:then_0
            (Utilities|IsValid (Variables|Default|GetSelectedUnit)
              (:Is%20Valid
                (Default|SetIsSelected (Variables|Default|GetSelectedUnit) false))))
          (:then_1
            (bind _output_get (Variables|Default|SetSelectedUnit (LocalVariables|GetNewUnit)))
            (Utilities|IsValid _output_get
              (:Is%20Valid
                (Default|SetIsSelected _output_get true)))))))))

(fn OnGridGenerated
  (if (Default|IsIndexValid (Variables|References|GetGrid) (Variables|Default|GetSelectedTile))
    (CallFunction|SetSelectedTileandUnit (Variables|Default|GetSelectedTile) true)
    (else
      (CallFunction|SetSelectedTileandUnit (Utilities|Struct|MakeIntPoint -999 -999) true))))

(fn OnTileDataUpdated
  (params (Index :type Int%20Point%20Structure))
  (if (Class|KismetMathLibrary|EqualIntPointIntPoint Index (Variables|Default|GetSelectedTile))
    (CallFunction|OnGridGenerated)))

(fn OnUnitGridIndexChanged
  (params (Unit :type BP%20Unit%20Object%20Reference))
  (if (== Unit (Variables|Default|GetSelectedUnit))
    (CallFunction|SetSelectedTileandUnit (Variables|/Game/Blueprints/Core/Units/BP_Unit.BP_Unit_C|GetIndex Unit) false)))