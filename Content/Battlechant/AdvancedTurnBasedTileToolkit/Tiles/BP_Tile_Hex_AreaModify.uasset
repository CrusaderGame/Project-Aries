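; Hex tile actor for the Advanced Turn Based Tile Toolkit that changes movement edge costs across an area of the grid.
; On BeginPlay it gathers the tiles within Range of its anchor's grid index and sets every existing edge between two of those tiles to NewCost in the GridManager.
; It refreshes the edge debug display if enabled, then destroys itself, acting as a one-shot level modifier.
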(event EventBeginPlay
  (bind _gridmanager (CallFunction|GetGridManager))
  (Development|PrintString "Hello--------------------------------------------------------")
  (bind _output_get (Variables|Default|SetCenterGrid (Variables|/Game/AdvancedTurnBasedTileToolkit/Core/BP_GridAnchor.BP_GridAnchor_C|GetGridIndex (Variables|Default|GetBP_GridAnchor))))
  (bind _insighttiles (Default|FindTilesinRange (.GridManager (CallFunction|GetGridManager)) _output_get (Variables|Default|GetRange) false false 9999999.0 1 false))
  (bind _result (Utilities|Set|ToArray _insighttiles))
  (bind _output_get_2 (Variables|Default|SetAllTiles _result))
  (for _array_element _output_get_2
    (if (.ReturnValue (Utilities|Map|Find (Variables|/Game/AdvancedTurnBasedTileToolkit/Core/Grid/BP_GridManager.BP_GridManager_C|GetGridEdges _gridmanager) _array_element))
      (bind _keys (Utilities|Map|Keys (Utilities|Struct|BreakFEdges (.Value (Utilities|Map|Find (Variables|/Game/AdvancedTurnBasedTileToolkit/Core/Grid/BP_GridManager.BP_GridManager_C|GetGridEdges _gridmanager) _array_element)))))
      (Variables|Default|SetOutputEdges (Utilities|Struct|BreakFEdges (.Value (Utilities|Map|Find (Variables|/Game/AdvancedTurnBasedTileToolkit/Core/Grid/BP_GridManager.BP_GridManager_C|GetGridEdges _gridmanager) _array_element))))
      (for _array_element_2 _keys
        (if (!= (Utilities|Array|FindItem (Variables|Default|GetAllTiles) _array_element_2) -1)
          (Utilities|Map|Add (Variables|Default|GetOutputEdges) _array_element_2 (Variables|Default|GetNewCost))))
      (Utilities|Map|Add (Variables|/Game/AdvancedTurnBasedTileToolkit/Core/Grid/BP_GridManager.BP_GridManager_C|GetGridEdges (.GridManager (CallFunction|GetGridManager))) _array_element (Utilities|Struct|MakeFEdges (Variables|Default|GetOutputEdges)))
      (Utilities|Map|Clear (Variables|Default|GetOutputEdges))))
  (if (Variables|/Game/AdvancedTurnBasedTileToolkit/Core/Grid/BP_GridManager.BP_GridManager_C|GetbDebugDisplayTileEdges _gridmanager)
    (Default|DisplayTileEdges _gridmanager))
  (Actor|DestroyActor))

(event Collision|EventActorBeginOverlap
  (params (OtherActor :type Actor%20Object%20Reference)))

(event EventTick
  (params (DeltaSeconds :type Float%20%28single-precision%29)))

(fn ConstructionScript
  (|CallParentFunction)
  (Variables|Default|SetDecalScale "1.000000,1.000000,1.000000")
  (Variables|Default|SetbShouldSetDecalScale true))