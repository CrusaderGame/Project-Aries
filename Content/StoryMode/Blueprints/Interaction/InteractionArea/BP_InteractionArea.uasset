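; BP_InteractionArea is a Story Mode interaction area that relays focus changes to its parent actor and the player's interact prompt.
; ToogleFocus stores the focused state and passes it to the parent actor through an interface message.
; It then shows or hides the WBPInteract widget on the story mode controller's UI and forwards the state to that widget's custom event.
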(event Custom|ToogleFocus
  (params (Focused :type Boolean))
  (bind _returnvalue (Game|GetPlayerController 0))
  (bind _asbp_story_mode_controller (Utilities|Casting|CastToBP_StoryModeController _returnvalue))
  (bind _ui (Variables|/Game/StoryMode/Blueprints/Core/BP_StoryModeController.BP_StoryModeController_C|GetUI _asbp_story_mode_controller))
  (bind _wbp_interact (Variables|/Game/StoryMode/UI/WBP_StoryModeUI.WBP_StoryModeUI_C|GetWBP_Interact _ui))
  (Variables|Default|SetFocused Focused)
  (Class|BPIInteraction|InterfaceToogleFocus(Message) (Actor|GetParentActor) (Variables|Default|GetFocused))
  (Widget|SetVisibility _wbp_interact (select (Variables|Default|GetFocused) "Visible" "Hidden"))
  (Default|CustomEvent _wbp_interact (Variables|Default|GetFocused)))

(fn ConstructionScript)