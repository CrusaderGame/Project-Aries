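; Interaction component for story mode that detects the BP_InteractionArea the player looks at and lets them interact with it.
; Every tick it line-traces on Visibility from player 0's follow camera, toggling focus on interaction areas as the hit actor changes.
; TryToInteract passes the focused area to InteractOnServer, which sends an interface interact message to that area's parent actor.
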(event Custom|TryToInteract
  (params (IN :type Boolean))
  (if IN
    (if (Variables|Default|GetIsTracingInteractionArea)
      (CallFunction|InteractonServer (Variables|Default|GetFocusedInteractionArea)))))

(event Custom|InteractOnServer
  (params (InteractionArea :type BP%20Interaction%20Area%20Object%20Reference))
  (Class|BPIInteraction|InterfaceInteract(Message) (Actor|GetParentActor InteractionArea)))

(event EventTick
  (params (DeltaSeconds :type Float%20%28single-precision%29))
  (CallFunction|Trace))

(fn Trace
  (bind _returnvalue (Game|GetPlayerCharacter 0))
  (bind _asbp_story_mode_character (Utilities|Casting|CastToBP_StoryModeCharacter _returnvalue))
  (bind _followcamera (Variables|/Game/StoryMode/Blueprints/Core/BP_StoryModeCharacter.BP_StoryModeCharacter_C|GetFollowCamera _asbp_story_mode_character))
  (bind _returnvalue_2 (Transformation|GetWorldLocation _followcamera))
  (bind (_outhit _returnvalue_3) (Collision|LineTraceByChannel _returnvalue_2 (+ _returnvalue_2 (* (Math|Vector|GetForwardVector _followcamera) (Variables|Default|GetLenght))) "TraceTypeQuery1" false 0 "None"))
  (if _returnvalue_3
    (if (!= (Variables|Default|GetFocusedActor) (.HitActor (Collision|BreakHitResult _outhit)))
      (Variables|Default|SetFocusedActor (.HitActor (Collision|BreakHitResult _outhit)))
      (CallFunction|TraceInteractionArea (== (Utilities|GetClass (.HitActor (Collision|BreakHitResult _outhit))) "/Game/StoryMode/Blueprints/Interaction/InteractionArea/BP_InteractionArea.BP_InteractionArea_C")))
    (else
      (CallFunction|TraceInteractionArea false))))

(fn TraceInteractionArea
  (params (Trace :type Boolean))
  (if Trace
    (if (Variables|Default|GetIsTracingInteractionArea)
      (Default|ToogleFocus (Variables|Default|GetFocusedInteractionArea) false))
    (bind _asbp_interaction_area (Utilities|Casting|CastToBP_InteractionArea (Variables|Default|GetFocusedActor)))
    (bind _output_get (Variables|Default|SetFocusedInteractionArea _asbp_interaction_area))
    (Default|ToogleFocus _output_get true)
    (Variables|Default|SetIsTracingInteractionArea true)
    (elif (Variables|Default|GetIsTracingInteractionArea)
      (Variables|Default|SetIsTracingInteractionArea false)
      (Default|ToogleFocus (Variables|Default|GetFocusedInteractionArea) false)
      (Variables|Default|SetFocusedActor 0)
      (Variables|Default|SetFocusedInteractionArea 0))))