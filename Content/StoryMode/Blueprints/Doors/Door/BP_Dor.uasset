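; BP_Dor is a story-mode door actor that registers itself with the player character when the player is within its Box trigger.
; Box overlap, plus a delayed check on BeginPlay for a player already inside, passes the door through SetNewDoorMessage; end overlap clears it for the leaving actor.
; SetCollisionDoor toggles collision on the door and both handles.
; No opening logic appears here, and the InteractToogle RepNotify and widget getter are empty stubs.
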(event OnComponentBeginOverlap(Box)
  (params (OverlappedComponent :type Primitive%20Component%20Object%20Reference) (OtherActor :type Actor%20Object%20Reference) (OtherComp :type Primitive%20Component%20Object%20Reference) (OtherBodyIndex :type Integer) (bFromSweep :type Boolean) (SweepResult :type Hit%20Result%20Structure%20%28by%20ref%29))
  (if (== OtherActor (Game|GetPlayerCharacter 0))
    (Class|BPIDoor|SetNewDoor(Message) OtherActor self)))

(event OnComponentEndOverlap(Box)
  (params (OverlappedComponent :type Primitive%20Component%20Object%20Reference) (OtherActor :type Actor%20Object%20Reference) (OtherComp :type Primitive%20Component%20Object%20Reference) (OtherBodyIndex :type Integer))
  (Class|BPIDoor|SetNewDoor(Message) OtherActor))

(event Custom|IsOverlapDoor
  (for _array_element (Collision|GetOverlappingActors (Variables|Default|GetBox) 0 :!class /Script/Engine.PrimitiveComponent)
    (if (== _array_element (Game|GetPlayerCharacter 0))
      (Class|BPIDoor|SetNewDoor(Message) _array_element self))))

(event Custom|AttachRightMouse
  (params (RughtHand :type Boolean))
  (Variables|Default|SetRught%20Hand RughtHand))

(event Custom|SetCollisionDoor
  (params (Collision :type Boolean))
  (if Collision
    (Collision|SetCollisionEnabled (Variables|Default|GetDoor) "QueryAndPhysics")
    (else
      (Collision|SetCollisionEnabled (Variables|Default|GetDoor) "NoCollision"))))

(event EventBeginPlay
  (bind _asbp_story_mode_character (Utilities|Casting|CastToBP_StoryModeCharacter (Game|GetPlayerCharacter 0)))
  (Variables|Default|SetCharacter _asbp_story_mode_character)
  (Utilities|FlowControl|Delay 0.2)
  (CallFunction|IsOverlapDoor))

(fn ConstructionScript)

(fn OnRepInteractToogle
  (if (Variables|Default|GetInteractToogle)
    _))

(fn GetInteractionWidgetRef
  (return 0))