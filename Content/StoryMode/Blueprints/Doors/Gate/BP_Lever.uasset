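; BP_Lever is an interactable, one-shot lever that opens the BP_Gate found in the level at BeginPlay.
; Focus toggles custom depth on its two meshes, and interaction flips InteractToogle through InteractOnServer.
; The OnRep of that flag, guarded by Usable, runs two timelines that animate the lever mesh and swing both gate doors open, then disables further use.
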(event Custom|InteractOnServer
  (Variables|Default|SetInteractToogle (not (Variables|Default|GetInteractToogle))))

(event Custom|OpenGate
  (bind _gate (Variables|Default|GetGate))
  (bind _floatvalue (Timeline|Timeline PlayFromStart)
    (:Update
      (Transformation|SetRelativeRotation (Variables|/Game/StoryMode/Blueprints/Doors/Gate/BP_Gate.BP_Gate_C|GetDoorL _gate) (Math|Rotator|MakeRotator 0.0 0.0 (Math|Float|Lerp 1.8e+02 2.8e+02 _floatvalue)) false false)
      (Transformation|SetRelativeRotation (Variables|/Game/StoryMode/Blueprints/Doors/Gate/BP_Gate.BP_Gate_C|GetDoorR _gate) (Math|Rotator|MakeRotator 0.0 0.0 (Math|Float|Lerp 1.8e+02 8e+01 _floatvalue)) false false))))

(event Custom|LeverUse
  (bind _floatvalue (Timeline|Timeline_0 PlayFromStart)
    (:Update
      (Transformation|SetRelativeLocationAndRotation (Variables|Default|GetStaticMesh1) (Math|Vector|MakeVector 0.0 (Math|Float|Lerp 25.0 5.0 _floatvalue) 46.224525) (Math|Rotator|MakeRotator 9e+01 (Math|Float|Lerp 1.2e+02 2.2e+02 _floatvalue) 9e+01) false false))))

(event EventInterfaceInteract
  (CallFunction|InteractonServer))

(event EventBeginPlay
  (bind _returnvalue (Actor|GetActorOfClass "/Game/StoryMode/Blueprints/Doors/Gate/BP_Gate.BP_Gate_C"))
  (Variables|Default|SetGate _returnvalue))

(event EventInterfaceToogleFocus
  (params (Focus :type Boolean))
  (Rendering|SetRenderCustomDepth (Variables|Default|GetStaticMesh) Focus))

(fn ConstructionScript)

(fn OnRepInteractToogle
  (if (Variables|Default|GetUsable?)
    (if (Variables|Default|GetInteractToogle)
      (CallFunction|LeverUse)
      (CallFunction|OpenGate)
      (Variables|Default|SetUsable? false))))

(fn GetInteractionWidgetRef
  (return 0))