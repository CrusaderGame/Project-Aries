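; BP_MainMenu runs the turn-based tactics game's main menu, creating the WBP_MainMenu widget on BeginPlay and adding it to the viewport.
; It then loops endlessly through streamed square, hexagon and triangle levels as an animated backdrop behind the menu.
; Each level loads without blocking while the widget shows the background, holds, then hides it before the level unloads and the next streams in.
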(event EventBeginPlay
  (bind _returnvalue (UserInterface|CreateWidget "/Game/TurnBasedTactic/Blueprints/Other/MainMenu/WBP_MainMenu.WBP_MainMenu_C"))
  (bind _output_get (Variables|Default|SetW_MainMenu _returnvalue))
  (UserInterface|Viewport|AddtoViewport _output_get 0)
  ;[0 0 0] [EN] Loop through the different levels so we have something interesting behind the main menu
  ; [FR] Passe à travers tous les levels pour qu'on ait quelque chose d'intéressant derrière le main menu
  (Game|LoadStreamLevel(byName) "L_Square" true :!label _label)
  (Default|EventShowBackground (Variables|Default|GetW_MainMenu))
  (Utilities|FlowControl|Delay 1e+01)
  (Default|EventHideBackground (Variables|Default|GetW_MainMenu))
  (Utilities|FlowControl|Delay 5.0)
  (Game|UnloadStreamLevel(byName) "L_Square" false)
  (Game|LoadStreamLevel(byName) "L_Hexagon" true)
  (Default|EventShowBackground (Variables|Default|GetW_MainMenu))
  (Utilities|FlowControl|Delay 1e+01)
  (Default|EventHideBackground (Variables|Default|GetW_MainMenu))
  (Utilities|FlowControl|Delay 5.0)
  (Game|UnloadStreamLevel(byName) "L_Hexagon" false)
  (Game|LoadStreamLevel(byName) "L_Triangle" true)
  (Default|EventShowBackground (Variables|Default|GetW_MainMenu))
  (Utilities|FlowControl|Delay 1e+01)
  (Default|EventHideBackground (Variables|Default|GetW_MainMenu))
  (Utilities|FlowControl|Delay 5.0)
  (Game|UnloadStreamLevel(byName) "L_Triangle" false)
  (goto _label))

(fn ConstructionScript)