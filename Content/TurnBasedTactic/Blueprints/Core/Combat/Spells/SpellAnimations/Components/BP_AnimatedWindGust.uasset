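; Spell animation actor that shows a green wind gust sliding from an origin transform to a target.
; Construction gives both mesh material slots translucent dynamic materials with randomized green brightness.
; On BeginPlay, a rate-adjusted timeline lerps the actor transform and drives material opacity.
; It signals shape animation completion once partway through playback, then destroys itself shortly after the timeline finishes.
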(event EventBeginPlay
  ;[0 0 0] [EN] Basic blueprint that sets the desired visual and then simply slides from the origin to the target.
  ; [FR] Blueprint de base qui applique le visuel voulu pour ensuite simplement glisser à partir de l'origin vers la target
  (Components|Timeline|SetPlayRate (Variables|Default|GetTimeline_PlayAnimation) (Variables|Default|GetPlayRate))
  (bind (_direction _transformalpha _opacity) (Timeline|Timeline_PlayAnimation PlayFromStart)
    (:Update
      (Transformation|SetActorTransform (Math|Transform|Lerp(Transform) (Variables|Default|GetOriginTransform) (Variables|Default|GetTargetTransform) _transformalpha))
      (Rendering|Material|SetScalarParameterValueonMaterials (Variables|Default|GetAnimatedWindGust) "Opacity" _opacity)
      (if (>= (Components|Timeline|GetPlaybackPosition (Variables|Default|GetTimeline_PlayAnimation)) 0.35)
        (Utilities|FlowControl|DoOnce false
          (:Completed
            (Default|CallOnShapeAnimationCompleted self)))))
    (:Finished
      (Utilities|FlowControl|Delay 0.5)
      (Actor|DestroyActor))))

(fn ConstructionScript
  (bind _returnvalue (Rendering|Material|CreateDynamicMaterialInstance (Variables|Default|GetAnimatedWindGust) 0 "/Game/TurnBasedTactic/Demo/Art/Materials/M_TranslucentColor.M_TranslucentColor" "None" :!class /Script/Engine.PrimitiveComponent))
  (Rendering|Material|SetVectorParameterValue _returnvalue "Color" (* "(R=0.045654,G=0.515625,B=0.082430,A=1.000000)" (Math|Random|RandomFloatinRange 0.8 1.5)) :!class /Script/Engine.MaterialInstanceDynamic)
  (bind _returnvalue_2 (Rendering|Material|CreateDynamicMaterialInstance (Variables|Default|GetAnimatedWindGust) 1 "/Game/TurnBasedTactic/Demo/Art/Materials/M_TranslucentColor.M_TranslucentColor" "None" :!class /Script/Engine.PrimitiveComponent))
  (Rendering|Material|SetVectorParameterValue _returnvalue_2 "Color" (* "(R=0.145833,G=1.000000,B=0.212673,A=1.000000)" (Math|Random|RandomFloatinRange 0.8 1.5)) :!class /Script/Engine.MaterialInstanceDynamic))