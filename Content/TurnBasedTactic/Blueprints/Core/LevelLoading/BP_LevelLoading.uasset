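; BP_LevelLoading streams one named sublevel at a time for the tactics game.
; LoadLevel hides and unloads the current streaming level, then loads and shows the requested one, skipping repeats unless forced and printing an error for invalid names other than None.
; BeginPlay force-loads the configured level, then repeats the call after a short delay as a workaround for nav mesh generation in 5.1.
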(event EventBeginPlay
  ;[0 0 0] [EN] Load level on BeginPlay
  ; [FR] Charge le niveau au BeginPlay
  (CallFunction|LoadLevel (Variables|Default|GetLevelLoaded) true)
  (Utilities|FlowControl|Delay 0.5) ; TODO : So nav mesh is generated properly in 5.1
  (CallFunction|LoadLevel (Variables|Default|GetLevelLoaded) true))

(fn ConstructionScript)

(fn LoadLevel
  (params (Level :type String) (Force :type Boolean))
  ;[0 0 0] [EN] Do not load the currently loaded level, unless you forced it
  ; [FR] Ne charge pas le niveau qui est déjà chargé, sauf si tu le force
  (if (or Force (Utilities|Enum|NotEqual(Enum) Level (Variables|Default|GetLevelLoaded)))
    (Utilities|FlowControl|Sequence
      (:then_0
        ;[0 0 0] [EN] Unload previous level
        ; [FR] Unload le level précédent
        (Utilities|IsValid (Class|GameplayStatics|GetStreamingLevel (Utilities|String|StringToName (Variables|Default|GetLevelLoaded)))
          (:Is%20Valid
            (Variables|/Script/Engine.LevelStreaming|SetbShouldBeLoaded (Class|GameplayStatics|GetStreamingLevel (Utilities|String|StringToName (Variables|Default|GetLevelLoaded))) false)
            (Variables|/Script/Engine.LevelStreaming|SetbShouldBeVisible (Class|GameplayStatics|GetStreamingLevel (Utilities|String|StringToName (Variables|Default|GetLevelLoaded))) false))))
      (:then_1
        ;[0 0 0] [EN] Then load the desired level
        ; [FR] Ensuite load le level désiré
        (bind _output_get (Variables|Default|SetLevelLoaded Level))
        (Utilities|IsValid (Class|GameplayStatics|GetStreamingLevel (Utilities|String|StringToName _output_get))
          (:Is%20Valid
            (Variables|/Script/Engine.LevelStreaming|SetbShouldBeLoaded (Class|GameplayStatics|GetStreamingLevel (Utilities|String|StringToName _output_get)) true)
            (Variables|/Script/Engine.LevelStreaming|SetbShouldBeVisible (Class|GameplayStatics|GetStreamingLevel (Utilities|String|StringToName _output_get)) true))
          (:Is%20Not%20Valid
            ;[0 0 0] [EN] If the desired level is invalid and not equal to ''None'', print an error message
            ; [FR] Si le level désiré n'est pas valide et qu'il n'est pas égal à ''None'', on print un message d'erreur
            (if (Utilities|Enum|NotEqual(Enum) (Variables|Default|GetLevelLoaded) "None")
              (Development|PrintString (Utilities|String|Append "Error - LoadLevel - Invalid Level Name: " (Variables|Default|GetLevelLoaded)) true true "(R=1.000000,G=0.000000,B=0.000000,A=1.000000)" 5.0))))))))