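; BP_PC is the player controller for a turn-based tactics game, acting as a relay for networked unit actions.
; On BeginPlay it caches the BP_PlayerActions actor and shows the mouse cursor.
; Its OnServer events forward movement, turn advance, HP changes, spell hits and death handling to multicast or plain events on the passed target.
; Only the HP change checks authority before forwarding.
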(event Custom|On%20Server%20Move%20Unit
  (params (Unit :type BP%20Unit%20Object%20Reference) (Path :type Array%20of%20Int%20Point%20Structures) (Target :type BP%20Combat%20System%20Object%20Reference))
  (Default|MulticastMoveUnit Target Unit Path))

(event Custom|On%20Server%20Next%20Unit
  (params (Target :type BP%20Combat%20System%20Object%20Reference))
  (Default|MulticastNextUnit Target))

(event Custom|On%20Server%20Modify%20Current%20Hp
  (params (Modifier :type Integer) (ShowNumber :type Boolean) (Target :type BP%20Unit%20Object%20Reference))
  ;[1 1 1] Do bana
  (Networking|SwitchHasAuthority
    (:Authority
      (Default|MulticastModifyCurrentHp Target Modifier ShowNumber))))

(event Custom|On%20Server%20Update%20Hp%20Bar
  (params (Target :type WBP%20Hp%20Bar%20Object%20Reference))
  ;[1 1 1] Do bana
  (Default|EventUpdateHpBar Target))

(event Custom|On%20Server%20Unit%20Hit%20by%20Spell
  (params (Target :type BP%20Unit%20Object%20Reference) (SpellAnimation :type BP%20Spell%20Animation%20Object%20Reference%20%28by%20ref%29) (SpellImpactReal :type S%20Spell%20Data%20Impact%20Real%20Structure%20%28by%20ref%29))
  (Default|MulticastUnitHitbySpell Target SpellAnimation SpellImpactReal))

(event Custom|On%20Server%20HideUnitAfterFewSeconds
  (params (Target :type BP%20Unit%20Object%20Reference))
  ;[1 1 1] Do bana
  (Default|EventHideUnitAfterFewSeconds Target))

(event Custom|On%20Server%20Process%20Unit%20Death
  (params (Target :type BP%20Combat%20System%20Object%20Reference) (Unit :type BP%20Unit%20Object%20Reference))
  (Default|MulticastProcessUnitDeath Target Unit))

(event EventBeginPlay
  (bind _returnvalue (Actor|GetActorOfClass "/Game/TurnBasedTactic/Blueprints/Core/Player/BP_PlayerActions.BP_PlayerActions_C"))
  (Variables|Default|SetPlayerActions _returnvalue)
  ;[0 0 0] [EN] When the game starts, we show the mouse cursor.
  ; [FR] Quand le jeu commence, on rend le curseur visible.
  (Variables|Default|SetbShowMouseCursor true))

(fn ConstructionScript)