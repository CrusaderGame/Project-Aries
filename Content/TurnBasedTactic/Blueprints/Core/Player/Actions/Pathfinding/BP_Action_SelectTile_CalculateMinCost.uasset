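; Player action that, after running its parent action, fills the grid's pathfinding data with each tile's minimum cost to the selected tile, for inspection with debug texts.
; On execute it clears the generated data and, if the selected tile is valid, discovers every grid tile through GridPathfinding.
; Cost from start is left at zero, and the minimum cost estimate respects the include-diagonals setting.
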(event EventBeginPlay
  (|CallParentFunction) ; This node is disabled and will not be called.\nDrag off pins to build functionality.
)

(event Collision|EventActorBeginOverlap
  (params (OtherActor :type Actor%20Object%20Reference))
  (|CallParentFunction OtherActor) ; This node is disabled and will not be called.\nDrag off pins to build functionality.
)

(event EventTick
  (params (DeltaSeconds :type Float%20%28single-precision%29))
  (|CallParentFunction DeltaSeconds) ; This node is disabled and will not be called.\nDrag off pins to build functionality.
)

(fn ConstructionScript
  (|CallParentFunction))

(fn ExecuteAction
  (params (Index :type Int%20Point%20Structure))
  (bind _playeractions (Variables|Default|GetPlayerActions))
  (bind _playeractions_2 (Variables|Default|GetPlayerActions))
  (bind _grid (Variables|/Game/TurnBasedTactic/Blueprints/Core/Player/BP_PlayerActions.BP_PlayerActions_C|GetGrid _playeractions_2))
  ;[0 0 0] [EN] Select Tile
  ; [FR] Sélectionne la case
  (|CallParentFunction Index)
  ;[0 0 0] [EN] Clear data before regenerating it
  ; [FR] Clear le data avant de le regénérer
  (Default|ClearGeneratedData (Variables|/Game/TurnBasedTactic/Blueprints/Core/Grid/BP_Grid.BP_Grid_C|GetGridPathfinding (Variables|/Game/TurnBasedTactic/Blueprints/Core/Player/BP_PlayerActions.BP_PlayerActions_C|GetGrid (Variables|Default|GetPlayerActions))))
  ;[0 0 0] [EN] Loop through all the tiles and discover them. Just to have some data to look at with the debug texts
  ; [FR] Loop à travers toutes les cases et les discover. Juste pour avoir du data qu'on peut regarder avec les debug textes
  (if (Default|IsIndexValid (Variables|/Game/TurnBasedTactic/Blueprints/Core/Player/BP_PlayerActions.BP_PlayerActions_C|GetGrid _playeractions) (Variables|/Game/TurnBasedTactic/Blueprints/Core/Player/BP_PlayerActions.BP_PlayerActions_C|GetSelectedTile _playeractions))
    (bind _keys (Utilities|Map|Keys (Variables|/Game/TurnBasedTactic/Blueprints/Core/Grid/BP_Grid.BP_Grid_C|GetGridTiles _grid)))
    (for _array_element _keys
      (Default|DiscoverTile (Variables|/Game/TurnBasedTactic/Blueprints/Core/Grid/BP_Grid.BP_Grid_C|GetGridPathfinding (Variables|/Game/TurnBasedTactic/Blueprints/Core/Player/BP_PlayerActions.BP_PlayerActions_C|GetGrid (Variables|Default|GetPlayerActions))) (Utilities|Struct|MakeS_PathfindingData _array_element 1 0 (Default|GetMinimumCostBetweenTwoTiles (Variables|/Game/TurnBasedTactic/Blueprints/Core/Grid/BP_Grid.BP_Grid_C|GetGridPathfinding _grid) _array_element (Variables|/Game/TurnBasedTactic/Blueprints/Core/Player/BP_PlayerActions.BP_PlayerActions_C|GetSelectedTile _playeractions_2) (Variables|Default|GetIncludeDiagonals)))))))