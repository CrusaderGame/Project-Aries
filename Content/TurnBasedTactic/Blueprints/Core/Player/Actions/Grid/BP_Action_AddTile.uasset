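; BP_Action_AddTile is a player grid action that adds a tile to the tactics grid at the given index.
; ExecuteAction only acts when that index is not already valid on the grid.
; It traces for the ground at the index's location so the new tile sits at floor height, then adds it with the grid's rotation and scale.
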(fn ConstructionScript
  (|CallParentFunction))

(fn ExecuteAction
  (params (Index :type Int%20Point%20Structure))
  (bind _playeractions (Variables|Default|GetPlayerActions))
  (bind _grid (Variables|/Game/TurnBasedTactic/Blueprints/Core/Player/BP_PlayerActions.BP_PlayerActions_C|GetGrid _playeractions))
  ;[0 0 0] [EN] We're only adding the tiles if they are not already there. And we make sure to trace for the ground so the new tile is properly aligned with the world
  ; [FR] On ajoute seulement une case si elle n'est pas déjà là. Et on trace pour le sol afin que la nouvelle case soit bien allignée avec la hauteur du plancher.
  (if (not (Default|IsIndexValid (Variables|/Game/TurnBasedTactic/Blueprints/Core/Player/BP_PlayerActions.BP_PlayerActions_C|GetGrid (Variables|Default|GetPlayerActions)) Index))
    (bind _outlocation (Default|TraceforGround (Variables|/Game/TurnBasedTactic/Blueprints/Core/Player/BP_PlayerActions.BP_PlayerActions_C|GetGrid (Variables|Default|GetPlayerActions)) (Default|GetTileLocationfromGridIndex _grid Index)))
    (Default|AddGridTile (Variables|/Game/TurnBasedTactic/Blueprints/Core/Player/BP_PlayerActions.BP_PlayerActions_C|GetGrid (Variables|Default|GetPlayerActions)) (Utilities|Struct|MakeS_TileData Index "NewEnumerator1" (Math|Transform|MakeTransform _outlocation (Default|GetTileRotationfromGridIndex _grid Index) (Default|GetTileScale _grid)) "NewEnumerator0"))))