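; AC_BedTime is a component that handles sleeping by jumping the DynomegaTimeOfDay clock to a chosen hour and minute.
; BedTime forwards the request to S_BedTime, which fires C_BedTime to show a fade, waits briefly, then calls JumpToNext on the time-of-day blueprint.
; C_BedTime adds a UI_BedTimeFade widget for the first player controller, gated by a DoOnce that resets after a short delay to prevent stacked fades.
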(event Custom|BedTime
  (params (Sleep%20Until%20Hour :type Integer) (Minute :type Integer))
  (CallFunction|SBedTime Sleep%20Until%20Hour Minute))

(event Custom|C_BedTime
  (Utilities|FlowControl|DoOnce false :!label _label
    (:Completed
      (bind _returnvalue (UserInterface|CreateWidget "/Game/DynomegaTimeOfDay/UIs/Bedtime/UI_BedTimeFade.UI_BedTimeFade_C" (Game|GetPlayerController 0)))
      (UserInterface|Viewport|AddtoViewport _returnvalue 0)
      (Utilities|FlowControl|Delay 1.0)
      (goto _label Reset))))

(event Custom|S_BedTime
  (params (Hour :type Integer) (Minute :type Integer))
  (CallFunction|CBedTime)
  (Utilities|FlowControl|Delay 0.6)
  (bind _timeofdaybp (CallFunction|GetTimeOfDayBP))
  (Default|JumptoNext _timeofdaybp Hour Minute))