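; Player controller component that relays server-side time-of-day events to the client UI.
; On BeginPlay it retries each tick until the TimeOfDay Blueprint is found, then binds its time, calendar and speed dispatchers.
; Each event passes through a client-side C_ event to UI dispatchers for the HUD.
; It also creates the time HUD and adds AC_BedTime to its owner if a bed exists and the component is missing.
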(event Custom|WaitForTimeOfDay
  ;[1 0.1722 0.04246] Initialize and Setup this Component
  (Utilities|FlowControl|DelayUntilNextTick)
  (bind (_timeofdaybp _found_) (CallFunction|GetTimeOfDayBP))
  (if _found_
    (Variables|Default|SetTime%20Of%20Day%20BP _timeofdaybp)
    (Utilities|FlowControl|Sequence
      (:then_0
        (CallFunction|SetupBindings))
      (:then_1
        (CallFunction|SetupTimeHUD))
      (:then_2
        (CallFunction|SetupBedtimeComponent)))
    (else
      (CallFunction|WaitforTimeOfDay))))

(event Custom|C_onNewMinute
  (params (TotalMinutes :type Float%20%28double-precision%29) (CurrentMinute :type Integer) (SecondsTracked :type Float%20%28double-precision%29) (DayPercent :type Float%20%28double-precision%29))
  ;[0.07292 0.07292 0.07292 1 24] These event dispatchers we are binding into are only sent from the server. If we hear something we relay it to our client for use in our UI. We do this because our UI does not have access to the server, and the server does not have access to our UI. The HUD binds into the events on this component to use the client side version of these event dispatchers.
  ;;[0.375 0.375 0.375 0.635] New Minute Detected
  (Default|CallUIonNewMinute (Utilities|DoubletoInt64PlusOne TotalMinutes) CurrentMinute (Utilities|DoubletoInt64PlusOne SecondsTracked) DayPercent))

(event Custom|onNewDay
  (params (TotalDays :type Integer) (DayInYear :type Integer) (DayOfWeekNumber :type Integer) (DayOfWeekName :type Text) (DayInMonth :type Integer) (MonthPercent :type Float%20%28double-precision%29) (Datestamp :type Text))
  ;[0.07292 0.07292 0.07292 1 24] These event dispatchers we are binding into are only sent from the server. If we hear something we relay it to our client for use in our UI. We do this because our UI does not have access to the server, and the server does not have access to our UI. The HUD binds into the events on this component to use the client side version of these event dispatchers.
  ;;[0.375 0.375 0.375 0.635] New Day Detected
  (CallFunction|ConNewDay TotalDays DayInYear DayOfWeekNumber DayOfWeekName DayInMonth MonthPercent Datestamp))

(event Custom|onNewWeek
  (params (TotalWeeks :type Integer))
  ;[0.07292 0.07292 0.07292 1 24] These event dispatchers we are binding into are only sent from the server. If we hear something we relay it to our client for use in our UI. We do this because our UI does not have access to the server, and the server does not have access to our UI. The HUD binds into the events on this component to use the client side version of these event dispatchers.
  ;;[0.375 0.375 0.375 0.635] New Week Detected
  (CallFunction|ConNewWeek TotalWeeks))

(event Custom|onNewMonth
  (params (TotalMonths :type Integer) (NewMonthName :type Text) (NewMonthNumberInYear :type Integer) (MonthStartDayInYear :type Integer) (DaysInMonth :type Integer))
  ;[0.07292 0.07292 0.07292 1 24] These event dispatchers we are binding into are only sent from the server. If we hear something we relay it to our client for use in our UI. We do this because our UI does not have access to the server, and the server does not have access to our UI. The HUD binds into the events on this component to use the client side version of these event dispatchers.
  ;;[0.375 0.375 0.375 0.635] New Month Detected
  (CallFunction|ConNewMonth TotalMonths NewMonthName NewMonthNumberInYear MonthStartDayInYear DaysInMonth))

(event Custom|onNewYear
  (params (TotalYears :type Integer))
  ;[0.07292 0.07292 0.07292 1 24] These event dispatchers we are binding into are only sent from the server. If we hear something we relay it to our client for use in our UI. We do this because our UI does not have access to the server, and the server does not have access to our UI. The HUD binds into the events on this component to use the client side version of these event dispatchers.
  ;;[0.375 0.375 0.375 0.635] New Year Detected
  (CallFunction|ConNewYear TotalYears))

(event Custom|SetupBindings
  ;[0.07292 0.07292 0.07292 1 24] These event dispatchers we are binding into are only sent from the server. If we hear something we relay it to our client for use in our UI. We do this because our UI does not have access to the server, and the server does not have access to our UI. The HUD binds into the events on this component to use the client side version of these event dispatchers.
  ;;[0.375 0.375 0.375 0.635] New Time of Day Detected
  (EventDispatchers|BindEventtoOnTimeOfDayChange (Variables|Default|GetTime%20Of%20Day%20BP) (delegate Custom|onTimeOfDayChange))
  ;;[0.375 0.375 0.375 0.635] New Minute Detected
  (EventDispatchers|BindEventtoOnNewMinute (Variables|Default|GetTime%20Of%20Day%20BP) (delegate Custom|onNewMinute))
  ;;[0.375 0.375 0.375 0.635] New Hour Detected
  (EventDispatchers|BindEventtoOnNewHour (Variables|Default|GetTime%20Of%20Day%20BP) (delegate Custom|onNewHour))
  ;;[0.375 0.375 0.375 0.635] New Day Detected
  (EventDispatchers|BindEventtoOnNewDay (Variables|Default|GetTime%20Of%20Day%20BP) (delegate Custom|onNewDay))
  ;;[0.375 0.375 0.375 0.635] New Week Detected
  (EventDispatchers|BindEventtoOnNewWeek (Variables|Default|GetTime%20Of%20Day%20BP) (delegate Custom|onNewWeek))
  ;;[0.375 0.375 0.375 0.635] New Month Detected
  (EventDispatchers|BindEventtoOnNewMonth (Variables|Default|GetTime%20Of%20Day%20BP) (delegate Custom|onNewMonth))
  ;;[0.375 0.375 0.375 0.635] New Year Detected
  (EventDispatchers|BindEventtoOnNewYear (Variables|Default|GetTime%20Of%20Day%20BP) (delegate Custom|onNewYear))
  ;;[0.375 0.375 0.375 0.635] New Speed Change Detected
  (EventDispatchers|BindEventtoOnSpeedChange (Variables|Default|GetTime%20Of%20Day%20BP) (delegate Custom|onSpeedChange)))

(event Custom|C_onNewHour
  (params (TotalHours :type Float%20%28double-precision%29) (CurrentHour :type Integer))
  ;[0.07292 0.07292 0.07292 1 24] These event dispatchers we are binding into are only sent from the server. If we hear something we relay it to our client for use in our UI. We do this because our UI does not have access to the server, and the server does not have access to our UI. The HUD binds into the events on this component to use the client side version of these event dispatchers.
  ;;[0.375 0.375 0.375 0.635] New Hour Detected
  (Default|CallUIonNewHour TotalHours CurrentHour))

(event Custom|SetupTimeHUD
  ;[0.07292 0.07292 0.07292] Attach our HUD
  (bind _returnvalue (UserInterface|CreateWidget "/Game/DynomegaTimeOfDay/UIs/TimeHUD/UI_TimeOfDayHUD.UI_TimeOfDayHUD_C" (Game|GetPlayerController 0) self))
  (bind _output_get (Variables|Default|SetUI_TimeOfDayHUD _returnvalue))
  (UserInterface|Viewport|AddtoViewport _output_get 0))

(event Custom|C_onSpeedChange
  (params (NewSpeed :type Float%20%28double-precision%29))
  ;[0.07292 0.07292 0.07292 1 24] These event dispatchers we are binding into are only sent from the server. If we hear something we relay it to our client for use in our UI. We do this because our UI does not have access to the server, and the server does not have access to our UI. The HUD binds into the events on this component to use the client side version of these event dispatchers.
  ;;[0.375 0.375 0.375 0.635] New Speed Change Detected
  (Default|CallUIonSpeedChange NewSpeed))

(event Custom|C_onTimeOfDayChange
  (params (TimeOfDay :type E_TimeOfDays%20Enum :default "NewEnumerator0"))
  ;[0.07292 0.07292 0.07292 1 24] These event dispatchers we are binding into are only sent from the server. If we hear something we relay it to our client for use in our UI. We do this because our UI does not have access to the server, and the server does not have access to our UI. The HUD binds into the events on this component to use the client side version of these event dispatchers.
  ;;[0.375 0.375 0.375 0.635] New Time of Day Detected
  (Default|CallUIonTimeOfDayChange TimeOfDay))

(event Custom|onTimeOfDayChange
  (params (TimeOfDay :type E_TimeOfDays%20Enum :default "NewEnumerator0"))
  ;[0.07292 0.07292 0.07292 1 24] These event dispatchers we are binding into are only sent from the server. If we hear something we relay it to our client for use in our UI. We do this because our UI does not have access to the server, and the server does not have access to our UI. The HUD binds into the events on this component to use the client side version of these event dispatchers.
  ;;[0.375 0.375 0.375 0.635] New Time of Day Detected
  (CallFunction|ConTimeOfDayChange TimeOfDay))

(event Custom|onSpeedChange
  (params (NewSpeed :type Float%20%28double-precision%29))
  ;[0.07292 0.07292 0.07292 1 24] These event dispatchers we are binding into are only sent from the server. If we hear something we relay it to our client for use in our UI. We do this because our UI does not have access to the server, and the server does not have access to our UI. The HUD binds into the events on this component to use the client side version of these event dispatchers.
  ;;[0.375 0.375 0.375 0.635] New Speed Change Detected
  (CallFunction|ConSpeedChange NewSpeed))

(event Custom|C_onNewDay
  (params (TotalDays :type Integer) (DayInYear :type Integer) (DayOfWeekNumber :type Integer) (DayOfWeekName :type Text) (DayInMonth :type Integer) (MonthPercent :type Float%20%28double-precision%29) (Datestamp :type Text))
  ;[0.07292 0.07292 0.07292 1 24] These event dispatchers we are binding into are only sent from the server. If we hear something we relay it to our client for use in our UI. We do this because our UI does not have access to the server, and the server does not have access to our UI. The HUD binds into the events on this component to use the client side version of these event dispatchers.
  ;;[0.375 0.375 0.375 0.635] New Day Detected
  (Default|CallUIonNewDay TotalDays DayInYear DayOfWeekNumber DayOfWeekName DayInMonth MonthPercent Datestamp))

(event Custom|C_onNewWeek
  (params (TotalWeeks :type Integer))
  ;[0.07292 0.07292 0.07292 1 24] These event dispatchers we are binding into are only sent from the server. If we hear something we relay it to our client for use in our UI. We do this because our UI does not have access to the server, and the server does not have access to our UI. The HUD binds into the events on this component to use the client side version of these event dispatchers.
  ;;[0.375 0.375 0.375 0.635] New Week Detected
  (Default|CallUIonNewWeek TotalWeeks))

(event Custom|C_onNewMonth
  (params (TotalMonths :type Integer) (NewMonthName :type Text) (NewMonthNumberInYear :type Integer) (MonthStartDayInYear :type Integer) (DaysInMonth :type Integer))
  ;[0.07292 0.07292 0.07292 1 24] These event dispatchers we are binding into are only sent from the server. If we hear something we relay it to our client for use in our UI. We do this because our UI does not have access to the server, and the server does not have access to our UI. The HUD binds into the events on this component to use the client side version of these event dispatchers.
  ;;[0.375 0.375 0.375 0.635] New Month Detected
  (Default|CallUIonNewMonth TotalMonths NewMonthName NewMonthNumberInYear MonthStartDayInYear DaysInMonth))

(event Custom|C_onNewYear
  (params (TotalYears :type Integer))
  ;[0.07292 0.07292 0.07292 1 24] These event dispatchers we are binding into are only sent from the server. If we hear something we relay it to our client for use in our UI. We do this because our UI does not have access to the server, and the server does not have access to our UI. The HUD binds into the events on this component to use the client side version of these event dispatchers.
  ;;[0.375 0.375 0.375 0.635] New Year Detected
  (Default|CallUIonNewYear TotalYears))

(event Custom|onNewMinute
  (params (TotalMinutes :type Float%20%28double-precision%29) (CurrentMinute :type Integer) (SecondsTracked :type Float%20%28double-precision%29) (DayPercent :type Float%20%28double-precision%29))
  ;[0.07292 0.07292 0.07292 1 24] These event dispatchers we are binding into are only sent from the server. If we hear something we relay it to our client for use in our UI. We do this because our UI does not have access to the server, and the server does not have access to our UI. The HUD binds into the events on this component to use the client side version of these event dispatchers.
  ;;[0.375 0.375 0.375 0.635] New Minute Detected
  (CallFunction|ConNewMinute TotalMinutes CurrentMinute SecondsTracked DayPercent))

(event Custom|SetupBedtimeComponent
  ;[0.07292 0.07292 0.07292] Add our bedtime component (for the UI) if we detect a bed in the world and the component is not already on our controller (the owner).
  ; If you are not using AC_TimeOfDayUI (this BP) but still want to use the bed UI you just need to add this AC_BedTime component to your controller manually.
  (bind _returnvalue (Actor|GetActorOfClass "/Game/DynomegaTimeOfDay/Blueprints/Utilities/BP_Bed.BP_Bed_C"))
  (Utilities|IsValid _returnvalue
    (:Is%20Valid
      (Utilities|IsValid (Actor|GetComponentbyClass (Components|GetOwner) "/Game/DynomegaTimeOfDay/Blueprints/Components/AC_BedTime.AC_BedTime_C")
        (:Is%20Not%20Valid
          (Game|AddComponentbyClass (Components|GetOwner) "/Game/DynomegaTimeOfDay/Blueprints/Components/AC_BedTime.AC_BedTime_C"))))))

(event Custom|onNewHour
  (params (TotalHours :type Float%20%28double-precision%29) (CurrentHour :type Integer))
  ;[0.07292 0.07292 0.07292 1 24] These event dispatchers we are binding into are only sent from the server. If we hear something we relay it to our client for use in our UI. We do this because our UI does not have access to the server, and the server does not have access to our UI. The HUD binds into the events on this component to use the client side version of these event dispatchers.
  ;;[0.375 0.375 0.375 0.635] New Hour Detected
  (CallFunction|ConNewHour TotalHours CurrentHour))

(event EventBeginPlay
  ;[1 0.1722 0.04246] Initialize and Setup this Component
  (bind (_timeofdaybp _found_) (CallFunction|GetTimeOfDayBP))
  (if _found_
    (Variables|Default|SetTime%20Of%20Day%20BP _timeofdaybp)
    (Utilities|FlowControl|Sequence
      (:then_0
        (CallFunction|SetupBindings))
      (:then_1
        (CallFunction|SetupTimeHUD))
      (:then_2
        (CallFunction|SetupBedtimeComponent)))
    (else
      (CallFunction|WaitforTimeOfDay))))