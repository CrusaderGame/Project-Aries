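; Spawner that places actors and runs a Niagara effect according to the world's time of day.
; On the authority it either reacts to time-of-day changes or checks fixed time windows each minute, spawning each fixed-time entry once per day.
; A shared handler applies spawn chance and global or tag-based live-count caps, tagging each spawned actor.
; The chosen Niagara system reaches clients through a RepNotify that swaps or deactivates the effect.
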(event Custom|onNewMinute
  (params (TotalMinutes :type Float%20%28double-precision%29) (CurrentMinute :type Integer) (SecondsTracked :type Float%20%28double-precision%29) (DayPercent :type Float%20%28double-precision%29))
  ;[0.07292 0.07292 0.07292] Setup Fixed Time Mode
  (CallFunction|FixedTimeSpawnNS)
  (CallFunction|FixedTimeSpawnActors))

(event Custom|onTimeOfDayChange
  (params (TimeOfDay :type E_TimeOfDays%20Enum :default "NewEnumerator0"))
  ;[0.07292 0.07292 0.07292] Setup Time of Day Mode
  (CallFunction|TimeOfDaySpawnNS TimeOfDay)
  (CallFunction|TimeOfDaySpawnActor TimeOfDay))

(event Custom|onNewDay
  (params (TotalDays :type Integer) (DayInYear :type Integer) (DayOfWeekNumber :type Integer) (DayOfWeekName :type Text) (DayInMonth :type Integer) (MonthPercent :type Float%20%28double-precision%29) (Datestamp :type Text))
  ;[0.07292 0.07292 0.07292] Setup Fixed Time Mode
  (Utilities|Array|Clear (Variables|Default|GetAlreadySpawnedActors)))

(event Custom|DeactivateNS
  ;[0.375 0.375 0.375 0.635] Niagara System Deactivator
  (Components|Activation|Deactivate (Variables|Default|GetNiagara)))

(event EventOnTimeOfDayLoaded
  ;[1 0.1722 0.04246] Setup Spawner
  (Networking|SwitchHasAuthority
    (:Authority
      (switch Utilities|FlowControl|Switch|SwitchonE_TimeOfDay_ScheduleTypes (Variables|Default|GetSwitchType)
        (:NewEnumerator0
          ;[0.07292 0.07292 0.07292] Setup Time of Day Mode
          (EventDispatchers|BindEventtoOnTimeOfDayChange (Variables|Default|GetBP_TimeOfDay) (delegate Custom|onTimeOfDayChange))
          (CallFunction|OnTimeOfDayChange (Default|GetTimeOfDay (Variables|Default|GetBP_TimeOfDay))))
        (:NewEnumerator1
          ;[0.07292 0.07292 0.07292] Setup Fixed Time Mode
          (EventDispatchers|BindEventtoOnNewMinute (Variables|Default|GetBP_TimeOfDay) (delegate Custom|onNewMinute))
          (EventDispatchers|BindEventtoOnNewDay (Variables|Default|GetBP_TimeOfDay) (delegate Custom|onNewDay)))))))

(fn ConstructionScript
  (|CallParentFunction))

(fn TimeOfDaySpawnNS
  (params (TimeOfDay :type E_TimeOfDays%20Enum%20%28by%20ref%29 :default "NewEnumerator0"))
  (bind _timeofdayniagarasystems (Variables|Default|TimeOfDaySwitch|GetTimeOfDayNiagaraSystems))
  (bind (_value _returnvalue) (Utilities|Map|Find _timeofdayniagarasystems TimeOfDay))
  (if _returnvalue
    (Variables|Default|SetCurrentNiagaraSystem _value)
    (else
      (Variables|Default|GetCurrentNiagaraSystem
        (:then
          (Variables|Default|SetCurrentNiagaraSystem 0))
        (:else)))))

(fn TimeOfDaySpawnActor
  (params (TimeOfDay :type E_TimeOfDays%20Enum%20%28by%20ref%29 :default "NewEnumerator0"))
  (bind _timeofdayactors (Variables|Default|TimeOfDaySwitch|GetTimeOfDayActors))
  (bind (_value _returnvalue) (Utilities|Map|Find _timeofdayactors TimeOfDay))
  ;[0.07292 0.07292 0.07292] See if each actor should be spawned
  (if _returnvalue
    (for _array_element (Utilities|Struct|BreakF_TimeOfDaySpawnActorsArray _value)
      (LocalVariables|SetspawnData _array_element)
      ;[0.07292 0.07292 0.07292] Get our actor tag
      (CallFunction|SpawnActorHandler (Utilities|GetTimeOfDaySpawnerActorTag TimeOfDay (Utilities|Struct|BreakF_TimeOfDaySpawnActor (LocalVariables|GetspawnData))) (LocalVariables|GetspawnData)))))

(fn FixedTimeSpawnNS
  (bind (_hour _minute) (Default|GetHourMinSec (Variables|Default|GetBP_TimeOfDay)))
  (LocalVariables|SetcurrentHour _hour)
  (LocalVariables|SetcurrentMinute _minute)
  (bind _keys (Utilities|Map|Keys (Variables|Default|FixedTimeSwitch|GetFixedTimeNiagaraSystems)))
  (for _array_element _keys
    (LocalVariables|SetthisNiagaraSystem _array_element)
    (if (CallFunction|IsInsideTimeWindow? (LocalVariables|GetcurrentHour) (LocalVariables|GetcurrentMinute) (.StartHour (Utilities|Struct|BreakF_TimeOfDaySchedule (.Value (Utilities|Map|Find (Variables|Default|FixedTimeSwitch|GetFixedTimeNiagaraSystems) (LocalVariables|GetthisNiagaraSystem))))) (.StartMinute (Utilities|Struct|BreakF_TimeOfDaySchedule (.Value (Utilities|Map|Find (Variables|Default|FixedTimeSwitch|GetFixedTimeNiagaraSystems) (LocalVariables|GetthisNiagaraSystem))))) (.EndHour (Utilities|Struct|BreakF_TimeOfDaySchedule (.Value (Utilities|Map|Find (Variables|Default|FixedTimeSwitch|GetFixedTimeNiagaraSystems) (LocalVariables|GetthisNiagaraSystem))))) (.EndMinute (Utilities|Struct|BreakF_TimeOfDaySchedule (.Value (Utilities|Map|Find (Variables|Default|FixedTimeSwitch|GetFixedTimeNiagaraSystems) (LocalVariables|GetthisNiagaraSystem))))))
      (if (not (Utilities|Array|ContainsItem (Variables|Default|GetRanNiagaraSystems) (LocalVariables|GetthisNiagaraSystem)))
        (Utilities|Array|Add (Variables|Default|GetRanNiagaraSystems) (LocalVariables|GetthisNiagaraSystem))
        (Variables|Default|SetCurrentNiagaraSystem (LocalVariables|GetthisNiagaraSystem)))
      (else
        (Utilities|FlowControl|Sequence
          (:then_0
            (if (Utilities|Array|ContainsItem (Variables|Default|GetRanNiagaraSystems) (LocalVariables|GetthisNiagaraSystem))
              (Utilities|Array|RemoveItem (Variables|Default|GetRanNiagaraSystems) (LocalVariables|GetthisNiagaraSystem))))
          (:then_1
            (if (== (Variables|Default|GetCurrentNiagaraSystem) (LocalVariables|GetthisNiagaraSystem))
              (Variables|Default|SetCurrentNiagaraSystem 0))))))))

(fn FixedTimeSpawnActors
  (bind (_hour _minute) (Default|GetHourMinSec (Variables|Default|GetBP_TimeOfDay)))
  (LocalVariables|SetcurrentHour _hour)
  (LocalVariables|SetcurrentMinute _minute)
  (bind _keys (Utilities|Map|Keys (Variables|Default|FixedTimeSwitch|GetFixedTimeActors)))
  (for (_array_element _array_index) _keys
    (LocalVariables|SetthisActor _array_element)
    (LocalVariables|SetthisActorIndex _array_index)
    (if (not (Utilities|Array|ContainsItem (Variables|Default|GetAlreadySpawnedActors) (LocalVariables|GetthisActorIndex)))
      (if (CallFunction|IsInsideTimeWindow? (LocalVariables|GetcurrentHour) (LocalVariables|GetcurrentMinute) (.StartHour (Utilities|Struct|BreakF_TimeOfDaySchedule (.Value (Utilities|Map|Find (Variables|Default|FixedTimeSwitch|GetFixedTimeActors) (LocalVariables|GetthisActor))))) (.StartMinute (Utilities|Struct|BreakF_TimeOfDaySchedule (.Value (Utilities|Map|Find (Variables|Default|FixedTimeSwitch|GetFixedTimeActors) (LocalVariables|GetthisActor))))) (.EndHour (Utilities|Struct|BreakF_TimeOfDaySchedule (.Value (Utilities|Map|Find (Variables|Default|FixedTimeSwitch|GetFixedTimeActors) (LocalVariables|GetthisActor))))) (.EndMinute (Utilities|Struct|BreakF_TimeOfDaySchedule (.Value (Utilities|Map|Find (Variables|Default|FixedTimeSwitch|GetFixedTimeActors) (LocalVariables|GetthisActor))))))
        (bind _spawnedsomething_ (CallFunction|SpawnActorHandler (Utilities|GetFixedTimeSpawnerActorTag (LocalVariables|GetthisActorIndex)) (LocalVariables|GetthisActor)))
        (if _spawnedsomething_
          (Utilities|Array|Add (Variables|Default|GetAlreadySpawnedActors) (LocalVariables|GetthisActorIndex)))))))

(fn SpawnActorHandler
  (params (Tag :type Name) (SpawnData :type F%20Time%20Of%20Day%20Spawn%20Actor%20Structure))
  (bind _maxactors (Utilities|Struct|BreakF_TimeOfDaySpawnActor SpawnData))
  (bind _actorblueprint (Utilities|Struct|BreakF_TimeOfDaySpawnActor SpawnData))
  (bind (_maxactors_2 _spawnallatonce_) (Utilities|Struct|BreakF_TimeOfDaySpawnActor SpawnData))
  (LocalVariables|SetthisTag Tag)
  (Utilities|FlowControl|Sequence
    (:then_0
      (|onSpawnChance SpawnData)
      (Utilities|FlowControl|Sequence
        (:then_0
          ;[0.07292 0.07292 0.07292] Determine if we should spawn this actor based on limitations
          (if (Utilities|Struct|BreakF_TimeOfDaySpawnActor SpawnData)
            (bind _outactors (Actor|GetAllActorsOfClass _actorblueprint))
            (bind _output_get (LocalVariables|SetLiveCount (Utilities|Array|Length _outactors)))
            (if (< _output_get _maxactors)
              (LocalVariables|SetspawnIt? true :!label _label))
            (else
              (bind _outactors_2 (Actor|GetAllActorsOfClasswithTag _actorblueprint (LocalVariables|GetthisTag)))
              (bind _output_get_2 (LocalVariables|SetLiveCount (Utilities|Array|Length _outactors_2)))
              (if (< _output_get_2 _maxactors)
                (goto _label)))))
        (:then_1
          ;[0.07292 0.07292 0.07292] Spawn the actor(s)
          (if (LocalVariables|GetspawnIt?)
            (if _spawnallatonce_
              (for _index (range 0 (Utilities|Operators|Subtract _maxactors_2 (LocalVariables|GetLiveCount) 1))
                (bind _returnvalue (Game|SpawnActorfromClass (Utilities|Struct|BreakF_TimeOfDaySpawnActor SpawnData) (Transformation|GetActorTransform) "Undefined" self 0))
                (Utilities|Array|AddUnique (Variables|/Script/Engine.Actor|GetTags _returnvalue) (LocalVariables|GetthisTag)))
              (else
                (bind _returnvalue_2 (Game|SpawnActorfromClass (Utilities|Struct|BreakF_TimeOfDaySpawnActor SpawnData) (Transformation|GetActorTransform) "Undefined" self 0))
                (Utilities|Array|AddUnique (Variables|/Script/Engine.Actor|GetTags _returnvalue_2) (LocalVariables|GetthisTag))))))))
    (:then_1
      (return (LocalVariables|GetspawnIt?)))))

(fn OnRepCurrentNiagaraSystem
  (if (== (Variables|Default|GetCurrentNiagaraSystem) 0)
    (CallFunction|DeactivateNS)
    (elif (Components|Activation|IsActive (Variables|Default|GetNiagara))
      (if (not (== (AssetData|GetAsset (Variables|Default|GetNiagara)) (Variables|Default|GetCurrentNiagaraSystem)))
        (Class|NiagaraComponent|SetAsset (Variables|Default|GetNiagara) (Variables|Default|GetCurrentNiagaraSystem) true :!label _label)
        (Components|Activation|SetActive (Variables|Default|GetNiagara) true true))
      (else
        (goto _label)))))