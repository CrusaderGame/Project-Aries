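; Time of Day utility actor that spins a set of actors in step with the time-of-day speed.
; When time of day loads, it binds to speed changes and adds a RotatingMovementComponent to any listed actor lacking one, using the base rotation rate.
; Speed changes set a RepNotify variable, whose OnRep scales the base rate by speed and applies it to those components.
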(event Custom|onSpeedChange
  (params (NewSpeed :type Float%20%28double-precision%29))
  (CallFunction|ConSpeedChange NewSpeed))

(event Custom|C_onSpeedChange
  (params (Speed :type Float%20%28double-precision%29))
  (Variables|Default|SetSpeed Speed))

(event EventOnTimeOfDayLoaded
  (EventDispatchers|BindEventtoOnSpeedChange (Variables|Default|GetBP_TimeOfDay) (delegate Custom|onSpeedChange))
  ;[0.07292 0.07292 0.07292] Add rotating movement component to actors without it.
  (for _array_element (Variables|Default|GetActorsToRotate)
    (Utilities|IsValid (Actor|GetComponentbyClass _array_element "/Script/Engine.RotatingMovementComponent")
      (:Is%20Not%20Valid
        (bind _returnvalue (Game|AddComponentbyClass _array_element "/Script/Engine.RotatingMovementComponent"))
        (Variables|/Script/Engine.RotatingMovementComponent|SetRotationRate _returnvalue (Math|Rotator|MakeRotator (.x (Variables|Default|GetRotationRate)) (.y (Variables|Default|GetRotationRate)) (.z (Variables|Default|GetRotationRate))))))))

(fn ConstructionScript
  (|CallParentFunction))

(fn OnRepSpeed
  ;[0.07292 0.07292 0.07292] Calculate our turn rate based on your speed
  (LocalVariables|SetTurnRate (* (Variables|Default|GetSpeed) (Variables|Default|GetRotationRate)))
  ;[0.07292 0.07292 0.07292] Apply turn rate to our actors
  (for _array_element (Variables|Default|GetActorsToRotate)
    (Utilities|IsValid (Actor|GetComponentbyClass _array_element "/Script/Engine.RotatingMovementComponent")
      (:Is%20Valid
        (Variables|/Script/Engine.RotatingMovementComponent|SetRotationRate (Actor|GetComponentbyClass _array_element "/Script/Engine.RotatingMovementComponent") (Math|Rotator|MakeRotator (.x (LocalVariables|GetTurnRate)) (.y (LocalVariables|GetTurnRate)) (.z (LocalVariables|GetTurnRate))))))))