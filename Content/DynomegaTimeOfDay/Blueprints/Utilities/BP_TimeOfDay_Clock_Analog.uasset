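; Analog clock actor for the Time of Day system that turns its hour and minute plates to show the current game time.
; It takes day percent from BP_TimeOfDay on load and each new minute, and the DayPercentage RepNotify triggers the clock update.
; The update converts day percent to 12-hour time and sets smooth fractional yaw rotations, guarded by a resettable DoOnce.
; The construction script applies configurable materials to case, loop, plate and hands.
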(event Custom|onNewMinute
  (params (TotalMinutes :type Float%20%28double-precision%29) (CurrentMinute :type Integer) (SecondsTracked :type Float%20%28double-precision%29) (DayPercent :type Float%20%28double-precision%29))
  ;[0.07292 0.07292 0.07292] Process our updates each minute
  (Variables|Default|SetDayPercentage DayPercent))

(event Custom|ResetNow
  ;[0.07292 0.07292 0.07292] Update Handler
  (Utilities|FlowControl|DoOnce false) ; enters at Reset
)

(event Custom|UpdateClock
  ;[0.07292 0.07292 0.07292] Update Handler
  (Utilities|FlowControl|DoOnce false
    (:Completed
      (CallFunction|UpdateAnalogClock))))

(event EventOnTimeOfDayLoaded
  (Utilities|FlowControl|Sequence
    (:then_0
      ;[0.07292 0.07292 0.07292] Get variables for rotation calculations
      (Variables|Default|SetSecondsPerMinute (Default|GetSecondsPerMinute (Variables|Default|GetBP_TimeOfDay)))
      (Variables|Default|SetMinutes%20Per%20Hour (Variables|/Game/DynomegaTimeOfDay/Blueprints/BP_TimeOfDay.BP_TimeOfDay_C|GetMinutesPerHour (Variables|Default|GetBP_TimeOfDay))))
    (:then_1
      (Variables|Default|SetDayPercentage (Default|GetDayPercent (Variables|Default|GetBP_TimeOfDay)))
      ;[0.07292 0.07292 0.07292] Process our updates each minute
      (EventDispatchers|BindEventtoOnNewMinute (Variables|Default|GetBP_TimeOfDay) (delegate Custom|onNewMinute)))))

(fn ConstructionScript
  (bind _hourhand (Variables|Default|GetHourHand))
  (bind _minutehand (Variables|Default|GetMinuteHand))
  (|CallParentFunction)
  (Rendering|Material|SetMaterial (Variables|Default|GetLoop) 0 (Variables|Default|GetLoopMaterial))
  (Rendering|Material|SetMaterial (Variables|Default|GetHourPlate) 0 (Variables|Default|GetPlateMaterial))
  (Rendering|Material|SetMaterial _hourhand 0 (Variables|Default|GetHourHandBallMaterial))
  (Rendering|Material|SetMaterial _hourhand 1 (Variables|Default|GetHourHandMaterial))
  (Rendering|Material|SetMaterial _minutehand 0 (Variables|Default|GetMinuteHandBallMaterial))
  (Rendering|Material|SetMaterial _minutehand 1 (Variables|Default|GetMinuteHandMaterial))
  (Rendering|Material|SetMaterial (Variables|Default|GetCase) 0 (Variables|Default|GetCaseMaterial)))

(fn OnRepDayPercentage
  (CallFunction|UpdateClock))

(fn UpdateAnalogClock
  (bind _bp_timeofday (Variables|Default|GetBP_TimeOfDay)
    (:then
      (bind (_hour _minute _second) (Default|GetHourMinSecfromDayPercent _bp_timeofday (Variables|Default|GetDayPercentage)))
      (Variables|Default|SetHour (CallFunction|To12Hour _hour))
      (Variables|Default|SetMinute _minute)
      (Variables|Default|SetSecond _second)
      (Transformation|SetRelativeRotation (Variables|Default|GetHourPlate) (Math|Rotator|MakeRotator 0.0 0.0 (* (/ (+ (Math|Conversions|ToFloat(Integer) (Variables|Default|GetHour)) (Math|Float|SafeDivide (+ (Math|Conversions|ToFloat(Integer) (Variables|Default|GetMinute)) (Math|Float|SafeDivide (Math|Conversions|ToFloat(Integer) (Variables|Default|GetSecond)) (Variables|Default|GetSecondsPerMinute))) (Variables|Default|GetMinutes%20Per%20Hour))) 12.0) 3.6e+02)) false false)
      (Transformation|SetRelativeRotation (Variables|Default|GetMinutePlate) (Math|Rotator|MakeRotator 0.0 0.0 (* (Math|Float|SafeDivide (+ (Math|Conversions|ToFloat(Integer) (Variables|Default|GetMinute)) (Math|Float|SafeDivide (Math|Conversions|ToFloat(Integer) (Variables|Default|GetSecond)) (Variables|Default|GetSecondsPerMinute))) (Variables|Default|GetMinutes%20Per%20Hour)) 3.6e+02)) false false)
      (CallFunction|ResetNow))
    (:else
      (CallFunction|ResetNow))))