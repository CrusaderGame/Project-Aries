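; Base Blueprint for Time of Day utilities that need a reference to the level's BP_TimeOfDay.
; On BeginPlay it looks up and caches that Blueprint, waits a tick, then fires the overridable OnTimeOfDayLoaded event.
; If the lookup fails it retries on following ticks, up to about ten times, then prints an error naming this utility.
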(event Custom|onTimeOfDayLoaded)

(event Custom|RetryLoadTimeOfDayBP
  (Utilities|FlowControl|DelayUntilNextTick) ; This gives our Time of day BP a chance to load.
  (bind (_timeofdaybp _found_) (CallFunction|GetTimeOfDayBP))
  (if _found_
    (Variables|Default|SetBP_TimeOfDay _timeofdaybp)
    (Utilities|FlowControl|DelayUntilNextTick)
    (CallFunction|OnTimeOfDayLoaded)
    (else
      (|RetryLoading))))

(event EventBeginPlay
  (bind (_timeofdaybp _found_) (CallFunction|GetTimeOfDayBP))
  (if _found_
    (Variables|Default|SetBP_TimeOfDay _timeofdaybp)
    (Utilities|FlowControl|DelayUntilNextTick)
    (CallFunction|OnTimeOfDayLoaded)
    (else
      (|RetryLoading))))

(fn ConstructionScript)