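; Base Blueprint for Time of Day utilities that switch in response to the Dynomega time-of-day system.
; Once Time of Day loads, SwitchType selects either Time Of Day mode, bound to time-of-day changes, or Fixed Time mode, bound to each new minute.
; Each mode fires once immediately, then forwards updates to empty OnChangeTimeOfDay or OnChangeMinute events that child classes override.
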(event Custom|onUtilityLoaded)

(event EventOnTimeOfDayLoaded
  (CallFunction|OnUtilityLoaded)
  (switch Utilities|FlowControl|Switch|SwitchonE_TimeOfDay_ScheduleTypes (Variables|Default|GetSwitchType)
    (:NewEnumerator0
      (|TimeOfDayMode))
    (:NewEnumerator1
      (|fixedTimeMode))))

(fn ConstructionScript
  (|CallParentFunction))

(event Custom|onChangeMinute)

(event Custom|C_onMinC
  (CallFunction|OnChangeMinute))

(event Custom|onMinC
  (params (TotalMinutes :type Float%20%28double-precision%29) (CurrentMinute :type Integer) (SecondsTracked :type Float%20%28double-precision%29) (DayPercent :type Float%20%28double-precision%29))
  (CallFunction|ConMinC))

(event Custom|C_onToDC
  (params (TimeOfDay :type E_TimeOfDays%20Enum :default "NewEnumerator0"))
  (CallFunction|OnChangeTimeOfDay TimeOfDay))

(event Custom|onChangeTimeOfDay
  (params (TimeOfDay :type E_TimeOfDays%20Enum :default "NewEnumerator0")))

(event Custom|onToDC
  (params (TimeOfDay :type E_TimeOfDays%20Enum :default "NewEnumerator0"))
  (CallFunction|ContoDC TimeOfDay))