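; Time-of-day switch that turns a list of other Blueprints on or off from the BPTimeOfDay clock.
; On load, SwitchType selects either a match against chosen time-of-day periods or a fixed hour-and-minute window.
; Time-of-day changes re-run the period check, and minute changes re-run the window check.
; Both checks set IsOn, whose RepNotify sends TurnOn or TurnOff messages to each valid listed Blueprint.
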(event Custom|onLoaded_1
  (switch Utilities|FlowControl|Switch|SwitchonE_TimeOfDay_ScheduleTypes (Variables|Default|GetSwitchType)
    (:NewEnumerator0
      (CallFunction|SetLightStatefromTimeOfDay (Default|GetTimeOfDay (Variables|Default|GetBP_TimeOfDay))))
    (:NewEnumerator1
      (CallFunction|SetLightStatefromFixedTime))))

(event EventOnChangeMinute
  (|CallParentFunction)
  (CallFunction|SetLightStatefromFixedTime))

(event EventOnChangeTimeOfDay
  (params (TimeOfDay :type E_TimeOfDays%20Enum :default "NewEnumerator0"))
  (|CallParentFunction TimeOfDay)
  (CallFunction|SetLightStatefromTimeOfDay TimeOfDay))

(fn ConstructionScript
  (|CallParentFunction))

(fn SetLightStatefromTimeOfDay
  (params (TimeOfDay :type E_TimeOfDays%20Enum :default "NewEnumerator0"))
  (Variables|Default|SetisOn? (Utilities|Array|ContainsItem (Variables|Default|GetTimeOfDayTurnOnAt) TimeOfDay)))

(fn SetLightStatefromFixedTime
  ;[0.07292 0.07292 0.07292] Are we in our window?
  (bind (_hour _minute) (Default|GetHourMinSec (Variables|Default|GetBP_TimeOfDay)))
  (if (CallFunction|IsInsideTimeWindow? _hour _minute (Variables|Default|GetFixedTimeTurnOnHour) (Variables|Default|GetFixedTimeTurnOnMinute) (Variables|Default|GetFixedTimeTurnOffHour) (Variables|Default|GetFixedTimeTurnOffMinute))
    (if (not (Variables|Default|GetisOn?))
      (Variables|Default|SetisOn? true))
    (elif (Variables|Default|GetisOn?)
      (Variables|Default|SetisOn? false))))

(fn OnRepIsOn?
  (for _array_element (Variables|Default|GetBlueprints)
    (Utilities|IsValid _array_element
      (:Is%20Valid
        (if (Variables|Default|GetisOn?)
          (Class|BPITimeOfDaySwitchRemote|Turnon(Message) _array_element)
          (else
            (Class|BPITimeOfDaySwitchRemote|TurnOff(Message) _array_element)))))))