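; Sky rotator actor for the time-of-day system that turns the level's directional lights as sun and moon.
; When time of day loads, it treats the brightest light as the sun, stores starting rotations, and removes duplicate rotators.
; A looping timer offsets each light's pitch by day percent around a fixed yaw path.
; It runs only on remote instances unless ChangeSkyOnServer is set, and warns about missing lights.
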(event Custom|onUpdateSky
  ;[0.07292 0.07292 0.07292] Setup our sky rotator
  (CallFunction|UpdateSky))

(event Custom|SetupSkyRotator
  ;[0.07292 0.07292 0.07292] Setup our sky rotator
  (if (Variables|Default|GetChangeSkyOnServer?)
    _
    (else
      (Networking|SwitchHasAuthority
        (:Remote
          _))))
  (CallFunction|SetStartingRotations)
  (Utilities|ContinueifLightsExist)
  (Utilities|Time|SetTimerbyEvent (delegate Custom|onUpdateSky) (Variables|Default|GetUpdateSkyRotationSpeed) true))

(event EventOnTimeOfDayLoaded
  (CallFunction|SetupSkyRotator)
  (|uniqueSkyRotatorCheck))

(fn ConstructionScript)

(fn UpdateSky
  (LocalVariables|SetCurrentDayOffset (* (Default|GetDayPercent (Variables|Default|GetBP_TimeOfDay)) 3.6e+02))
  (bind _keys (Utilities|Map|Keys (Variables|Default|GetStartingRotations)))
  (for _array_element _keys
    (Transformation|SetActorRotation _array_element (Math|Rotator|CombineRotators (Math|Rotator|MakeRotator 0.0 (|calculatePitch _array_element (LocalVariables|GetCurrentDayOffset)) (Variables|Default|GetSkyRotationPath)) "0, 0, 0"))))

(fn SetStartingRotations
  ;[0.07292 0.07292 0.07292] Get and validate our lights
  (bind _outactors (Actor|GetAllActorsOfClass "/Script/Engine.DirectionalLight"))
  (bind _output_get (LocalVariables|SetfoundDirectionalLights _outactors))
  (|ValidateLights _output_get
    (:Continue
      ;[0.07292 0.07292 0.07292] Get the intensity for all of our directional lights, whichever has the highest intensity we will treat as our sun.
      (for (_array_element _array_index) (LocalVariables|GetfoundDirectionalLights)
        (if (> (Variables|/Script/Engine.LightComponentBase|GetIntensity (Variables|/Script/Engine.Light|GetLightComponent _array_element)) (LocalVariables|GetCurrentMaxIntensityValue))
          (LocalVariables|SetCurrentMaxIntensityValue (Variables|/Script/Engine.LightComponentBase|GetIntensity (Variables|/Script/Engine.Light|GetLightComponent _array_element)))
          (LocalVariables|SetCurrentMaxIntensityIndex _array_index)))
      ;[0.07292 0.07292 0.07292] Set the starting rotations
      (for (_array_element_2 _array_index_2) (LocalVariables|GetfoundDirectionalLights)
        (Utilities|Map|Add (Variables|Default|GetStartingRotations) _array_element_2 (|getRotationForDirectionalLightByIndex (== _array_index_2 (LocalVariables|GetCurrentMaxIntensityIndex))))))))