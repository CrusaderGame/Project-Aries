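; Time-of-day switch that changes the color of its connected lights as the game clock advances.
; Minute changes check fixed-time color windows, while time-of-day changes look up a color in a map.
; Both paths set the RepNotify NewColor, whose notify runs a timeline fading all lights to it, starting from the first light's current color.
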(event Custom|UpdateLights
  ;[0.07292 0.07292 0.07292] If we have lights ...
  (if (Utilities|Array|IsNotEmpty (Variables|Default|GetConnectedLights))
    ;[0.07292 0.07292 0.07292] Get our current color
    (Variables|Default|SetBeforeColor (Rendering|Components|Light|GetLightColor (Variables|/Script/Engine.Light|GetLightComponent (Utilities|Array|Get(acopy) (Variables|Default|GetConnectedLights)))))
    ;[0.07292 0.07292 0.07292] Fade to our new color
    (bind _newtrack_0 (Timeline|3SecFloatTrack PlayFromStart)
      (:Update
        (CallFunction|SetLightColor (Math|Color|Lerp(LinearColor) (Variables|Default|GetBeforeColor) (Variables|Default|GetNewColor) _newtrack_0))))))

(event EventOnChangeMinute
  ;[0.07292 0.07292 0.07292] Switch Handlers
  (CallFunction|SetColorsBasedonFixedTime))

(event EventOnChangeTimeOfDay
  (params (TimeOfDay :type E_TimeOfDays%20Enum :default "NewEnumerator0"))
  ;[0.07292 0.07292 0.07292] Switch Handlers
  (CallFunction|SetColorsBasedonTimeOfDay TimeOfDay))

(fn ConstructionScript
  (|CallParentFunction))

(fn SetLightColor
  (params (NewLightColor :type Linear%20Color%20Structure))
  (for _array_element (Variables|Default|GetConnectedLights)
    (Rendering|Components|Light|SetLightColor (Variables|/Script/Engine.Light|GetLightComponent _array_element) NewLightColor true)))

(fn SetColorsBasedonTimeOfDay
  (params (Key :type E_TimeOfDays%20Enum%20%28by%20ref%29 :default "NewEnumerator0"))
  (bind _timeofdaycolors (Variables|Default|GetTimeOfDayColors))
  (bind (_value _returnvalue) (Utilities|Map|Find _timeofdaycolors Key))
  (if _returnvalue
    (Variables|Default|SetNewColor _value)))

(fn SetColorsBasedonFixedTime
  ;[0.07292 0.07292 0.07292] Check each schedule to see if any of them are in our window, if found see if it is not the current, and if it isn't set it as the new one
  (bind (_hour _minute) (Default|GetHourMinSec (Variables|Default|GetBP_TimeOfDay)))
  (for _array_element (Variables|Default|GetFixedTimeColors)
    (if (!= (.Color (Utilities|Struct|BreakF_TimeOfDay_ColorSchedule _array_element)) (Variables|Default|GetNewColor))
      (if (CallFunction|IsInsideTimeWindow? _hour _minute (.StartHour (Utilities|Struct|BreakF_TimeOfDay_ColorSchedule _array_element)) (.StartMinute (Utilities|Struct|BreakF_TimeOfDay_ColorSchedule _array_element)) (.EndHour (Utilities|Struct|BreakF_TimeOfDay_ColorSchedule _array_element)) (.EndMinute (Utilities|Struct|BreakF_TimeOfDay_ColorSchedule _array_element)))
        (Variables|Default|SetNewColor (.Color (Utilities|Struct|BreakF_TimeOfDay_ColorSchedule _array_element)))))))

(fn OnRepNewColor
  (CallFunction|UpdateLights))