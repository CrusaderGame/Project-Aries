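; Time of day utility that switches placed ambient sounds as the in-game clock changes, by either time-of-day period or fixed time windows.
; Minute and time-of-day change events pick the ActiveSound from the matching map, clearing it when a fixed window ends.
; Its RepNotify fades in the active sound and fades out the others in the set chosen by SwitchType.
; All assigned sounds are stopped when the utility loads.
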(event EventOnChangeMinute
  ;[0.07292 0.07292 0.07292] Switch Handlers
  (CallFunction|SetAmbientSoundbyFixedTime))

(event EventOnChangeTimeOfDay
  (params (TimeOfDay :type E_TimeOfDays%20Enum :default "NewEnumerator0"))
  ;[0.07292 0.07292 0.07292] Switch Handlers
  (CallFunction|SetAmbientSoundbyTimeOfDay TimeOfDay))

(event EventOnUtilityLoaded
  ;[0.07292 0.07292 0.07292] Stop all assigned sounds on load
  (CallFunction|StopAllAmbientSounds))

(fn ConstructionScript
  (|CallParentFunction))

(fn OnRepActiveSound
  ;[0.07292 0.07292 0.07292] Get our Ambient Sounds based on our switch type
  (switch Utilities|FlowControl|Switch|SwitchonE_TimeOfDay_ScheduleTypes (Variables|Default|GetSwitchType)
    (:NewEnumerator0
      (bind _values (Utilities|Map|Values (Variables|Default|GetTimeOfDayAmbientSounds)))
      (LocalVariables|SetambientSounds _values))
    (:NewEnumerator1
      (bind _keys (Utilities|Map|Keys (Variables|Default|GetFixedTimeAmbientSounds)))
      (LocalVariables|SetambientSounds _keys)))
  ;[0.07292 0.07292 0.07292] Fade in our Fade out our sound based on the updated value
  (for _array_element (LocalVariables|GetambientSounds)
    (if (!= (Variables|Default|GetActiveSound) _array_element)
      (if (Audio|Components|Audio|IsPlaying (Variables|/Script/Engine.AmbientSound|GetAudioComponent _array_element))
        (Audio|Components|Audio|FadeOut (Variables|/Script/Engine.AmbientSound|GetAudioComponent _array_element) (Variables|Default|GetFadeDuration) 0.0 "Linear" :!class /Script/Engine.AudioComponent))
      (elif (not (Audio|Components|Audio|IsPlaying (Variables|/Script/Engine.AmbientSound|GetAudioComponent _array_element)))
        (Audio|Components|Audio|FadeIn (Variables|/Script/Engine.AmbientSound|GetAudioComponent _array_element) (Variables|Default|GetFadeDuration) 1.0 0.0 "Linear" :!class /Script/Engine.AudioComponent)))))

(fn SetAmbientSoundbyTimeOfDay
  (params (Key :type E_TimeOfDays%20Enum%20%28by%20ref%29 :default "NewEnumerator0"))
  (bind _timeofdayambientsounds (Variables|Default|GetTimeOfDayAmbientSounds))
  (bind (_value _returnvalue) (Utilities|Map|Find _timeofdayambientsounds Key))
  (if (!= (Variables|Default|GetActiveSound) _value)
    (Variables|Default|SetActiveSound (select _returnvalue _value 0))))

(fn SetAmbientSoundbyFixedTime
  ;[0.07292 0.07292 0.07292] Get our current time
  (bind (_hour _minute) (Default|GetHourMinSec (Variables|Default|GetBP_TimeOfDay)))
  (LocalVariables|SetthisHour _hour)
  (LocalVariables|SetthisMinute _minute)
  ;[0.07292 0.07292 0.07292] Iterate through each ambient sound in our map
  (bind _keys (Utilities|Map|Keys (Variables|Default|GetFixedTimeAmbientSounds)))
  (for _array_element _keys
    (LocalVariables|SetthisAmbientSound _array_element)
    ;[0.07292 0.07292 0.07292] Are we in our window for this ambient sound?
    (if (CallFunction|IsInsideTimeWindow? (LocalVariables|GetthisHour) (LocalVariables|GetthisMinute) (.StartHour (Utilities|Struct|BreakF_TimeOfDaySchedule (.Value (Utilities|Map|Find (Variables|Default|GetFixedTimeAmbientSounds) (LocalVariables|GetthisAmbientSound))))) (.StartMinute (Utilities|Struct|BreakF_TimeOfDaySchedule (.Value (Utilities|Map|Find (Variables|Default|GetFixedTimeAmbientSounds) (LocalVariables|GetthisAmbientSound))))) (.EndHour (Utilities|Struct|BreakF_TimeOfDaySchedule (.Value (Utilities|Map|Find (Variables|Default|GetFixedTimeAmbientSounds) (LocalVariables|GetthisAmbientSound))))) (.EndMinute (Utilities|Struct|BreakF_TimeOfDaySchedule (.Value (Utilities|Map|Find (Variables|Default|GetFixedTimeAmbientSounds) (LocalVariables|GetthisAmbientSound))))))
      ;[0.07292 0.07292 0.07292] Is this ambient sound not the current one?
      (if (!= (LocalVariables|GetthisAmbientSound) (Variables|Default|GetActiveSound))
        ;[0.07292 0.07292 0.07292] Set New Sound
        (Variables|Default|SetActiveSound (LocalVariables|GetthisAmbientSound)))
      (else
        ;[0.07292 0.07292 0.07292] If we are outside our window but still playing stop it.
        (if (Audio|Components|Audio|IsPlaying (Variables|/Script/Engine.AmbientSound|GetAudioComponent (LocalVariables|GetthisAmbientSound)))
          ;[0.07292 0.07292 0.07292] Unset sound
          (if (== (LocalVariables|GetthisAmbientSound) (Variables|Default|GetActiveSound))
            (Variables|Default|SetActiveSound 0)))))))

(fn StopAllAmbientSounds
  (Utilities|FlowControl|Sequence
    (:then_0
      (bind _values (Utilities|Map|Values (Variables|Default|GetTimeOfDayAmbientSounds)))
      (bind _output_get (LocalVariables|SetAmbientSounds _values))
      (bind _keys (Utilities|Map|Keys (Variables|Default|GetFixedTimeAmbientSounds)))
      (Utilities|Array|AppendArray _output_get _keys))
    (:then_1
      (for _array_element (LocalVariables|GetAmbientSounds)
        (Utilities|IsValid _array_element
          (:Is%20Valid
            (Audio|Components|Audio|Stop (Variables|/Script/Engine.AmbientSound|GetAudioComponent _array_element))))))))