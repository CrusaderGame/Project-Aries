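; Time-of-day utility Blueprint that switches a set of connected lights on and off.
; Minute changes test a fixed on/off time window, while time-of-day changes check membership in a list of turn-on periods.
; Both update the IsLightOn RepNotify variable, whose OnRep sets visibility on every connected light.
; On utility load, the starting state is read from the first connected light's visibility.
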(event EventOnChangeMinute
  ;[0.07292 0.07292 0.07292] Switch Handlers
  (CallFunction|SetLightStatefromFixedTime))

(event EventOnChangeTimeOfDay
  (params (TimeOfDay :type E_TimeOfDays%20Enum :default "NewEnumerator0"))
  ;[0.07292 0.07292 0.07292] Switch Handlers
  (CallFunction|SetLightStatefromTimeOfDay TimeOfDay))

(event EventOnUtilityLoaded
  ;[0.07292 0.07292 0.07292] Get our starting state of the light
  (if (Utilities|Array|IsNotEmpty (Variables|Default|GetConnectedLights))
    (Variables|Default|SetisLightOn? (Rendering|IsVisible (Variables|/Script/Engine.Light|GetLightComponent (Utilities|Array|Get(acopy) (Variables|Default|GetConnectedLights)))))))

(fn ConstructionScript
  (|CallParentFunction))

(fn SetLightStatefromTimeOfDay
  (params (TimeOfDay :type E_TimeOfDays%20Enum :default "NewEnumerator0"))
  (Variables|Default|SetisLightOn? (Utilities|Array|ContainsItem (Variables|Default|GetTimeOfDayTurnOnAt) TimeOfDay)))

(fn SetLightStatefromFixedTime
  ;[0.07292 0.07292 0.07292] Are we in our window?
  (bind (_hour _minute) (Default|GetHourMinSec (Variables|Default|GetBP_TimeOfDay)))
  (if (CallFunction|IsInsideTimeWindow? _hour _minute (Variables|Default|GetFixedTimeTurnOnHour) (Variables|Default|GetFixedTimeTurnOnMinute) (Variables|Default|GetFixedTimeTurnOffHour) (Variables|Default|GetFixedTimeTurnOffMinute))
    (if (not (Variables|Default|GetisLightOn?)) ; Is the light still off?
      (Variables|Default|SetisLightOn? true))
    (elif (Variables|Default|GetisLightOn?) ; Is the light still on?
      (Variables|Default|SetisLightOn? false))))

(fn OnRepIsLightOn?
  (for _array_element (Variables|Default|GetConnectedLights)
    (Rendering|SetVisibility (Variables|/Script/Engine.Light|GetLightComponent _array_element) (Variables|Default|GetisLightOn?) false)))