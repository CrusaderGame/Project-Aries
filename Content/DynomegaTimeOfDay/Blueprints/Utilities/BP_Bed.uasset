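; BP_Bed is a bed prop that triggers sleeping until a configurable hour and minute when a player walks into its overlap sphere.
; The overlap finds the AC_BedTime component on the player controller and calls BedTime, printing a setup warning if it is missing.
; Construction applies configurable blanket, mattress and pillow materials.
; Blanket physics is switched off one second after BeginPlay, letting it settle first.
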(event OnComponentBeginOverlap(Sphere)
  (params (OverlappedComponent :type Primitive%20Component%20Object%20Reference) (OtherActor :type Actor%20Object%20Reference) (OtherComp :type Primitive%20Component%20Object%20Reference) (OtherBodyIndex :type Integer) (bFromSweep :type Boolean) (SweepResult :type Hit%20Result%20Structure%20%28by%20ref%29))
  (bind _asplayer_controller (Utilities|Casting|CastToPlayerController (Game|GetInstigatorController OtherActor)))
  (Utilities|IsValid (Actor|GetComponentbyClass _asplayer_controller "/Game/DynomegaTimeOfDay/Blueprints/Components/AC_BedTime.AC_BedTime_C")
    (:Is%20Valid
      (Default|BedTime (Actor|GetComponentbyClass _asplayer_controller "/Game/DynomegaTimeOfDay/Blueprints/Components/AC_BedTime.AC_BedTime_C") (Variables|Default|GetSleepUntilHour) (Variables|Default|GetSleepUntilMinute)))
    (:Is%20Not%20Valid
      (Development|PrintString " 
It looks like you are trying to use the bed but did not add the AC_BedTime 
component to your player controller. You will need to do that before the 
bed will work.  
 
View the documentation for more information." true true "(R=0.000000,G=0.845111,B=1.000000,A=1.000000)" 15.0))))

(event EventBeginPlay
  ;[0.07292 0.07292 0.07292] Disable physics
  (Utilities|FlowControl|Delay 1.0)
  (Physics|SetSimulatePhysics (Variables|Default|GetBlanket) false))

(fn ConstructionScript
  (Rendering|Material|SetMaterial (Variables|Default|GetBlanket) 0 (Variables|Default|GetBlanketMaterial))
  (Rendering|Material|SetMaterial (Variables|Default|GetMattress) 0 (Variables|Default|GetMattressMaterial))
  (Rendering|Material|SetMaterial (Variables|Default|GetPillow) 0 (Variables|Default|GetPillowMaterial)))