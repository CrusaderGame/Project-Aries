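; Digital clock actor that displays the current time of day from BPTimeOfDay on front and back text components, with optional AM/PM.
; Once time of day loads, it takes the initial timestamp and binds to the new-minute event to refresh it.
; The timestamp is a RepNotify variable, so changes replicate and update both texts through UpdateClock.
; The construction script previews default text with configurable color and size.
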(event Custom|onMinuteChanged
  (params (TotalMinutes :type Float%20%28double-precision%29) (CurrentMinute :type Integer) (SecondsTracked :type Float%20%28double-precision%29) (DayPercent :type Float%20%28double-precision%29))
  ;[0.07292 0.07292 0.07292] Update our clock on each new minute
  (bind _output_get (Variables|Default|SetCachedTimestamp (Default|GetTimestampfromSeconds (Variables|Default|GetBP_TimeOfDay) false (Variables|Default|GetShowAMPM?) SecondsTracked)))
  (if (Utilities|Enum|NotEqual(Enum) _output_get (Variables|Default|GetTimestampText))
    (Variables|Default|SetTimestampText (Variables|Default|GetCachedTimestamp))
    (else
      (CallFunction|UpdateClock))))

(event Custom|UpdateClock
  ;[0.07292 0.07292 0.07292] Show current value on our clock
  (Variables|Default|GetBP_TimeOfDay
    (:then
      (Rendering|Components|TextRender|SetText (Variables|Default|GetTimestamp) (Variables|Default|GetTimestampText)))
    (:else)))

(event EventOnTimeOfDayLoaded
  ;[0.07292 0.07292 0.07292] Set our value on load
  (Variables|Default|SetTimestampText (Default|GetTimestamp (Variables|Default|GetBP_TimeOfDay) false (Variables|Default|GetShowAMPM?)))
  ;[0.07292 0.07292 0.07292] Update our clock on each new minute
  (EventDispatchers|BindEventtoOnNewMinute (Variables|Default|GetBP_TimeOfDay) (delegate Custom|onMinuteChanged)))

(fn ConstructionScript
  (|CallParentFunction)
  (Variables|Default|SetDefaultText (Utilities|Text|FormatText "{default}{ampm}" (Variables|Default|GetDefaultText) (select (Variables|Default|GetShowAMPM?) " AM" "")))
  (Rendering|Components|TextRender|SetTextRenderColor (Variables|Default|GetTimestamp) (Variables|Default|GetTextColor))
  (Rendering|Components|TextRender|SetText (Variables|Default|GetTimestamp) (Variables|Default|GetDefaultText))
  (Rendering|Components|TextRender|SetWorldSize (Variables|Default|GetTimestamp) (Variables|Default|GetTextSize)))

(fn OnRepTimestampText
  (CallFunction|UpdateClock))