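; Shared helper functions for the Time of Day system, covering actor lookup and clock formatting.
; Getters find the BP_TimeOfDay actor by class or tag and report whether it is valid.
; Formatters convert hours to 12-hour and AM/PM forms and add ordinal suffixes to numbers through a map lookup defaulting to "th".
; A time-window check compares hours and minutes inclusively, handling ranges that cross midnight.
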(fn GetTimeOfDayBP
  (bind _returnvalue (Actor|GetActorOfClass 0 "/Game/DynomegaTimeOfDay/Blueprints/BP_TimeOfDay.BP_TimeOfDay_C"))
  (return _returnvalue (Utilities|IsValid _returnvalue)))

(fn GetTimeOfDayBPTagged
  (params (Tag :type Name))
  (bind _outactors (Actor|GetAllActorsOfClasswithTag 0 "/Game/DynomegaTimeOfDay/Blueprints/BP_TimeOfDay.BP_TimeOfDay_C" Tag))
  (return (Utilities|Array|Get(acopy) _outactors) (Utilities|IsValid (Utilities|Array|Get(acopy) _outactors))))

(fn GetOrdinal
  (params (Number :type Integer))
  (bind _ordinals (LocalVariables|GetOrdinals))
  (bind _ordinalnumber (|getOrdinalNumber Number))
  (bind (_value _returnvalue) (Utilities|Map|Find _ordinals _ordinalnumber))
  (return (Utilities|Text|FormatText "{number}{ordinal}" Number (select _returnvalue _value "th"))))

(fn GetAMPM
  (params (Hour :type Integer))
  (LocalVariables|SetcurrentHour Hour)
  (Utilities|FlowControl|Sequence
    (:then_0
      (if (> (LocalVariables|GetcurrentHour) 12) ; We only change the hour if it is greater then 12.
        (LocalVariables|SetampmText "PM")
        (LocalVariables|SetcurrentHour (- (LocalVariables|GetcurrentHour) 12))
        (else
          (LocalVariables|SetampmText (select (== (LocalVariables|GetcurrentHour) 12) "PM" "AM"))
          (if (== (LocalVariables|GetcurrentHour) 0)
            (LocalVariables|SetcurrentHour 12)))))
    (:then_1
      (return (LocalVariables|GetcurrentHour) (LocalVariables|GetampmText)))))

(fn IsInsideTimeWindow?
  (params (CurrentHour :type Integer) (CurrentMinute :type Integer) (StartHour :type Integer) (StartMinute :type Integer) (EndHour :type Integer) (EndMinute :type Integer))
  (if (> StartHour EndHour) ; Is our off time the next day?
    (if (or (> CurrentHour StartHour) (and (== CurrentHour StartHour) (>= CurrentMinute StartMinute))) ; Should we turn it on?
      (return true)
      (else
        (return (or (< CurrentHour EndHour) (and (== CurrentHour EndHour) (<= CurrentMinute EndMinute))))))
    (else
      (return (and (or (> CurrentHour StartHour) (and (== CurrentHour StartHour) (>= CurrentMinute StartMinute))) (or (< CurrentHour EndHour) (and (== CurrentHour EndHour) (<= CurrentMinute EndMinute))))))))

(fn To12Hour
  (params (Hour :type Integer))
  (return (select (> Hour 12) (- Hour 12) Hour)))