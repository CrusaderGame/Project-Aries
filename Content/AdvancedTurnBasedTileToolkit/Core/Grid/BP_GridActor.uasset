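; BP_GridActor is an actor that holds a position on the tile grid of the Advanced Turn Based Tile Toolkit.
; Its construction script looks up the grid manager and, if one is valid, runs the BPGridAnchor's external construction logic and copies the anchor's grid index.
; It exposes getting and setting of that index, and delegates placing the actor at its anchor to BPGridAnchor.
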(event EventSetGridIndex
  (params (GridIndex :type Integer))
  (Variables|Default|SetGridIndex GridIndex))

(fn ConstructionScript
  (bind _gridmanager (CallFunction|GetGridManager))
  (bind _bp_gridanchor (Variables|Default|GetBP_GridAnchor))
  (Utilities|IsValid _gridmanager
    (:Is%20Valid
      (Variables|Default|SetGridManagerRef _gridmanager)
      (Default|ExternalConstuctionScript _bp_gridanchor)
      (Variables|Default|SetGridIndex (Variables|/Game/AdvancedTurnBasedTileToolkit/Core/BP_GridAnchor.BP_GridAnchor_C|GetGridIndex _bp_gridanchor)))))

(fn PlaceActoratAnchor
  (Default|PlaceActoratAnchor (Variables|Default|GetBP_GridAnchor))
  (return))

(fn GetGridIndex
  (return true (Variables|Default|GetGridIndex)))