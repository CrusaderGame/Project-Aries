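; BP_GridAnchor is a scene component in the turn-based tile toolkit that anchors its owning actor to the grid.
; ExternalConstuctionScript conditionally snaps the component to the GridManager's closest traced tile at the owner's location and caches that tile's GridIndex.
; PlaceActorAtAnchor snaps the component to its closest tile plus AnchorOffset, moves the owner there, then zeroes the component's relative location.
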(event Custom|ExternalConstuctionScript
  (bind _gridmanager (CallFunction|GetGridManager))
  (bind _returnvalue (Components|GetOwner))
  (Utilities|IsValid _gridmanager
    (:Is%20Valid
      (if (or (Variables|Default|GetbIgnoreSnapToCustomGrid) (not (Default|CheckforCompileError _gridmanager)))
        _
        (else
          (bind _snaplocation (Default|FindClosestTiletoSnaptoTrace _gridmanager (Transformation|GetActorLocation _returnvalue) (Utilities|Array|MakeArray _returnvalue)))
          (Transformation|SetWorldLocation self _snaplocation false false)))
      (Variables|Default|SetGridIndex (Default|ConvertLocationtoIndex3DNaive _gridmanager _snaplocation)))))

(fn PlaceActoratAnchor
  (bind _snaplocation (Default|FindClosestTiletoSnaptoTrace (.GridManager (CallFunction|GetGridManager)) (Transformation|GetWorldLocation) (Utilities|Array|MakeArray (Components|GetOwner))))
  (Transformation|SetWorldLocation (+ _snaplocation (Variables|Default|GetAnchorOffset)) false false)
  (Transformation|SetActorLocation (Components|GetOwner) (Transformation|GetWorldLocation) false false)
  (Transformation|SetRelativeLocation "0, 0, 0" false false)
  (return))