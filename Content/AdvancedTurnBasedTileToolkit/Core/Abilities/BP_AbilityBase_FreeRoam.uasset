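; Free-roam movement ability for a unit in the turn-based tile toolkit, sending it to a clicked tile.
; Activation caches the owning actor as a BP_Unit, logging an error if the cast fails.
; On click release over a valid tile, ServerInteract pathfinds from the puppet's current location within the unit's max search range.
; If the tile is reachable and unoccupied, the unit moves there and the turn manager runs its post-ability step.
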(event EventActivate
  (params (bReassess :type Boolean) (OwningActor :type Actor%20Object%20Reference))
  (|CallParentFunction bReassess OwningActor)
  (bind _asbp_unit (Utilities|Casting|CastToBP_Unit OwningActor)
    (:then
      (Variables|Default|SetOwningUnit _asbp_unit))
    (:CastFailed
      (CallFunction|PrintErrorMessage "NewEnumerator0" "Failed to Cast BP_Unit"))))

(event EventServerInteract
  (params (bValidTile :type Boolean) (ClickedIndex :type Integer) (Location :type Vector :default "0, 0, 0") (Key :type Key%20Structure :default "None") (bReleased :type Boolean) (ClickType :type EClickType%20Enum :default "NewEnumerator0") (CallingPc :type BP%20Player%20Controller%20ATBTT%20Object%20Reference))
  (bind _owningunit (Variables|Default|GetOwningUnit))
  (if bValidTile
    (if bReleased
      (bind (_bfoundatleastone _foundgridindexes _pathsmap) (Default|RunPathfindingUntilIndexFound (Variables|Default|GetGridManagerRef) (Default|ConvertLocationtoIndex3DNaive (Variables|Default|GetGridManagerRef) (Transformation|GetActorLocation (Variables|/Game/AdvancedTurnBasedTileToolkit/Core/Units/BP_Unit.BP_Unit_C|GetPuppet (Variables|Default|GetOwningUnit)))) (Variables|/Game/AdvancedTurnBasedTileToolkit/Core/Units/BP_Unit.BP_Unit_C|GetMaxSearchRange _owningunit) (Variables|/Game/AdvancedTurnBasedTileToolkit/Core/Units/BP_Unit.BP_Unit_C|GetPathfindingType _owningunit) (Utilities|Array|MakeArray ClickedIndex)))
      (if _bfoundatleastone
        (if (not (Utilities|Map|Contains (Variables|/Game/AdvancedTurnBasedTileToolkit/Core/Grid/BP_GridManager.BP_GridManager_C|GetGridUnits (Variables|Default|GetGridManagerRef)) (Utilities|Array|Get(acopy) _foundgridindexes)))
          (Default|MovetoIndex (Variables|Default|GetOwningUnit) _pathsmap (Utilities|Array|Get(acopy) _foundgridindexes))
          (Default|RunAfterAbilityExecute (.TurnManager (CallFunction|GetTurnManager))))))))

(fn ConstructionScript
  (|CallParentFunction))