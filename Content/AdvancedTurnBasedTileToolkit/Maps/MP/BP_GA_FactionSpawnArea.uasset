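; BP_GA_FactionSpawnArea is an actor that visually marks a faction's spawn area in the multiplayer maps of the turn-based tile toolkit.
; The construction script scales a decal's Y and Z axes from SpawnRange and sets a text label to the faction name.
; It tints the decal through a dynamic material instance with a color selected by faction.
; BeginPlay only calls the parent, and GridManagerRef is unused.
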(event EventBeginPlay
  (|CallParentFunction))

(fn ConstructionScript
  (bind _spawnrange (Variables|Default|GetSpawnRange))
  (bind _returnvalue (Math|Conversions|ToFloat(Integer) _spawnrange))
  (bind _returnvalue_2 (+ _returnvalue 0.5))
  (|CallParentFunction)
  (Transformation|SetRelativeScale3D (Variables|Default|GetDecal) (Math|Vector|MakeVector 1.0 _returnvalue_2 _returnvalue_2))
  (Rendering|Components|TextRender|SetText (Variables|Default|GetTextRender) (Utilities|Text|ToText(String) (Utilities|String|EnumtoString (Variables|Default|GetFaction))))
  (bind _returnvalue_3 (Rendering|Material|CreateDynamicMaterialInstance (Variables|Default|GetDecal) :!class /Script/Engine.DecalComponent))
  (Rendering|Material|SetVectorParameterValue _returnvalue_3 "Color" (Utilities|Select :Index (Variables|Default|GetFaction) :NewEnumerator3 "" :NewEnumerator4 "(R=0.291667,G=0.291667,B=0.291667,A=1.000000)" :NewEnumerator0 "(R=0.103516,G=0.312500,B=0.073115,A=1.000000)" :NewEnumerator1 "(R=0.458333,G=0.157552,B=0.157552,A=1.000000)" :NewEnumerator5 "") :!class /Script/Engine.MaterialInstanceDynamic))