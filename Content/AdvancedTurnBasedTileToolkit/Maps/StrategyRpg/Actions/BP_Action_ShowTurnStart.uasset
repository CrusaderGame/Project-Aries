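; BP_Action_ShowTurnStart is a turn-based toolkit action that shows the turn start animation in the strategy RPG map's HUD.
; When played, it casts the player HUD to BP_HUD_ATBTT_Stats_Srpg and calls the layout widget's turn start animation with the current Turn, with a short delay before and after.
; It then ends the action, also doing so after printing an error if the HUD cast fails.
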(event EventPlayAction
  (bind _asbp_hud_atbtt_stats_srpg (Utilities|Casting|CastToBP_HUD_ATBTT_Stats_Srpg (HUD|GetHUD (Game|GetPlayerController 0)))
    (:then
      (Utilities|FlowControl|Delay 1.0)
      (Default|PlayTurnStartAnimation (Variables|/Game/AdvancedTurnBasedTileToolkit/Maps/StrategyRpg/Core/BP_HUD_ATBTT_Stats_Srpg.BP_HUD_ATBTT_Stats_Srpg_C|GetHommLayoutRef _asbp_hud_atbtt_stats_srpg) (Variables|Default|GetTurn))
      (Utilities|FlowControl|Delay 1.0)
      (CallFunction|EndAction true))
    (:CastFailed
      (CallFunction|PrintErrorMessage "NewEnumerator0" "Failed to Cast BP_HUD_ATBTT_Stats_Srpg")
      (CallFunction|EndAction true))))

(fn ConstructionScript
  (|CallParentFunction))