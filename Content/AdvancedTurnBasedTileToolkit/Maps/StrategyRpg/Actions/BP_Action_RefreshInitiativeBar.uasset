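; BP_Action_RefreshInitiativeBar is a queued action in the turn-based toolkit's strategy RPG map that updates the on-screen initiative bar.
; When played, it casts the first player controller's HUD to the SRPG stats HUD and passes its Puppets to the initiative bar widget in the Homm layout.
; It ends immediately afterward, logging an error first if the HUD cast fails.
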(event EventPlayAction
  (bind _asbp_hud_atbtt_stats_srpg (Utilities|Casting|CastToBP_HUD_ATBTT_Stats_Srpg (HUD|GetHUD (Game|GetPlayerController 0)))
    (:then
      (Default|RefreshInitiativeBar (Variables|/Game/AdvancedTurnBasedTileToolkit/Maps/StrategyRpg/UI/WBP_Layout_Srpg.WBP_Layout_Srpg_C|GetWBP_InitiativeBar (Variables|/Game/AdvancedTurnBasedTileToolkit/Maps/StrategyRpg/Core/BP_HUD_ATBTT_Stats_Srpg.BP_HUD_ATBTT_Stats_Srpg_C|GetHommLayoutRef _asbp_hud_atbtt_stats_srpg)) (Variables|Default|GetPuppets))
      (CallFunction|EndAction true))
    (:CastFailed
      (CallFunction|PrintErrorMessage "NewEnumerator0" "Failed to Cast BP_HUD_ATBTT_Stats_Srpg")
      (CallFunction|EndAction true))))

(fn ConstructionScript
  (|CallParentFunction))