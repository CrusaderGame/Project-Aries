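; HUD for the strategy RPG map of the Advanced Turn Based Tile Toolkit that opens with dialogue before the match begins.
; Its ClientInitialize override shows only the dialogue widget, deferring the parent initialization.
; OnDialogueCompletion removes that widget, runs the parent setup, adds the SRPG layout widget and asks the turn manager to attempt to start the match.
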(event Custom|OnDialogueCompletion
  (bind _dialoguepointer (Variables|Default|GetDialoguePointer))
  (if (Utilities|IsValid _dialoguepointer)
    (Widget|RemovefromParent _dialoguepointer))
  (|CallParentFunction)
  (bind _returnvalue (UserInterface|CreateWidget "/Game/AdvancedTurnBasedTileToolkit/Maps/StrategyRpg/UI/WBP_Layout_Srpg.WBP_Layout_Srpg_C" (Game|GetPlayerController 0)))
  (bind _output_get (Variables|Default|SetHommLayoutRef _returnvalue))
  (UserInterface|Viewport|AddtoViewport _output_get 0)
  (Default|AttemptStartMatch (.TurnManager (CallFunction|GetTurnManager))))

(event EventClientInitialize
  (bind _returnvalue (UserInterface|CreateWidget "/Game/AdvancedTurnBasedTileToolkit/Maps/StrategyRpg/UI/WBP_Dialogue.WBP_Dialogue_C" (Game|GetPlayerController 0)))
  (UserInterface|Viewport|AddtoViewport _returnvalue 0)
  (Variables|Default|SetDialoguePointer _returnvalue))

(fn ConstructionScript
  (|CallParentFunction))