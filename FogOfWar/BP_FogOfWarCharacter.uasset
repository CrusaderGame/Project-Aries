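; Character for a fog of war system that gives the player line-of-sight vision.
; On BeginPlay, two LineOfSight components start Visibility line traces and begin building their meshes.
; An older, disconnected system remains: LoSVisionSystem writes the player position to a material parameter collection, traces a forward cone, and draws the hits as a canvas triangle fan into a render target.
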(event EventTick
  (params (DeltaSeconds :type Float%20%28single-precision%29)))

(event EventBeginPlay
  (bind _lineofsight0 (Variables|Default|GetLineOfSight0))
  (Utilities|FlowControl|Sequence
    (:then_0
      (Class|LineOfSightComponent|StartLineTrace _lineofsight0 "TraceTypeQuery1" 60)
      (Class|LineOfSightComponent|StartLineTrace (Variables|Default|GetLineOfSight1) "TraceTypeQuery1" 60)
      (Class|LineOfSightComponent|StartBuildMesh _lineofsight0))))

(fn ConstructionScript)

(fn LoSVisionSystem
  (bind _los_render_target (Variables|Default|GetLoS%20Render%20Target))
  (Utilities|FlowControl|Sequence
    (:then_0
      (Rendering|Material|SetVectorParameterValue "/Game/FogOfWarV2/PlayrPosition.PlayrPosition" "PlayerPosition" (Math|Conversions|ToLinearColor(Vector) (Transformation|GetActorLocation)) :!class /Script/Engine.KismetMaterialLibrary))
    (:then_1
      (CallFunction|CreateCone))
    (:then_2
      (CallFunction|PrepareTrianglesforCanvas))
    (:then_3
      (Rendering|ClearRenderTarget2D _los_render_target)
      (bind (_canvas _size _context) (Rendering|BeginDrawCanvastoRenderTarget _los_render_target))
      (Class|Canvas|DrawTriangle _canvas 0 (Variables|Default|GetCanvasTriangles))
      (Rendering|EndDrawCanvastoRenderTarget _context))))

(fn CreateCone
  (bind _returnvalue (Transformation|GetActorLocation))
  (bind _traceresult (Variables|Default|GetTraceResult))
  (Utilities|Array|Clear (Variables|Default|GetTraceResult))
  (for _index (range 0 (Variables|Default|GetNumTraces))
    (bind (_outhit _returnvalue_2) (Collision|LineTraceByChannel _returnvalue (+ (* (Math|Vector|RotateVector (Math|Vector|RotateVector (Transformation|GetActorForwardVector) (Math|Rotator|MakeRotator 0.0 0.0 (/ (* (Variables|Default|GetNumTraces) (Variables|Default|GetDegreesPerTrace)) -2.0))) (Math|Rotator|MakeRotator 0.0 0.0 (* _index (Variables|Default|GetDegreesPerTrace)))) 7e+02) _returnvalue) "TraceTypeQuery1" false 0 "None"))
    (if _returnvalue_2
      (Utilities|Array|Add _traceresult (+ (* (Math|Vector|RotateVector (Math|Vector|RotateVector (Transformation|GetActorForwardVector) (Math|Rotator|MakeRotator 0.0 0.0 (/ (* (Variables|Default|GetNumTraces) (Variables|Default|GetDegreesPerTrace)) -2.0))) (Math|Rotator|MakeRotator 0.0 0.0 (* _index (Variables|Default|GetDegreesPerTrace)))) "") (.location _outhit)))
      (else
        (Utilities|Array|Add _traceresult (+ (* (Math|Vector|RotateVector (Math|Vector|RotateVector (Transformation|GetActorForwardVector) (Math|Rotator|MakeRotator 0.0 0.0 (/ (* (Variables|Default|GetNumTraces) (Variables|Default|GetDegreesPerTrace)) -2.0))) (Math|Rotator|MakeRotator 0.0 0.0 (* _index (Variables|Default|GetDegreesPerTrace)))) "") (+ (* (Math|Vector|RotateVector (Math|Vector|RotateVector (Transformation|GetActorForwardVector) (Math|Rotator|MakeRotator 0.0 0.0 (/ (* (Variables|Default|GetNumTraces) (Variables|Default|GetDegreesPerTrace)) -2.0))) (Math|Rotator|MakeRotator 0.0 0.0 (* _index (Variables|Default|GetDegreesPerTrace)))) 7e+02) _returnvalue)))))))

(fn PrepareTrianglesforCanvas
  (bind _returnvalue (Transformation|GetActorLocation))
  (bind _returnvalue_2 (Math|Vector|MakeVector 9e+02 9e+02 0.0))
  (bind _traceresult (Variables|Default|GetTraceResult))
  (Utilities|Array|Clear (Variables|Default|GetCanvasTriangles))
  (for _index (range 0 (- (Utilities|Array|Length (Variables|Default|GetTraceResult)) 2))
    (Utilities|Array|Add (Variables|Default|GetCanvasTriangles) (Utilities|Struct|MakeCanvasUVTri (Math|Conversions|ToVector2D(Vector) _returnvalue_2) "(X=0.000000,Y=0.000000)" "(R=1.000000,G=1.000000,B=1.000000,A=0.000000)" (Math|Conversions|ToVector2D(Vector) (+ (- (Utilities|Array|Get(acopy) _traceresult _index) _returnvalue) _returnvalue_2)) "(X=0.000000,Y=0.000000)" "(R=1.000000,G=1.000000,B=1.000000,A=0.000000)" (Math|Conversions|ToVector2D(Vector) (+ (- (Utilities|Array|Get(acopy) _traceresult (+ _index 1)) _returnvalue) _returnvalue_2)) "(X=0.000000,Y=0.000000)" "(R=1.000000,G=1.000000,B=1.000000,A=0.000000)"))))